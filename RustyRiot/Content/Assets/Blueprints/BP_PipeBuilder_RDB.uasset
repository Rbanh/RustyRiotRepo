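; Spline-based pipe builder that assembles a pipe along PipePath in the construction script.
; It resizes PipeData to the spline point count, places optional joint meshes with per-point roll, and stretches a spline mesh between neighboring points.
; AddObjectData places extra meshes at fractions of spline length with offset rotation and scale, aimed along the curve by sampling just ahead.
; An optional debug toggle labels each point with its index.
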(event EventBeginPlay)

(event Collision|EventActorBeginOverlap
  (params (OtherActor :type Actor%20Object%20Reference)))

(event EventTick
  (params (DeltaSeconds :type Float%20%28single-precision%29)))

(fn ConstructionScript
  (bind _pipe_data (Variables|Default|GetPipe_Data))
  (bind _pipepath (Variables|Default|GetPipePath))
  (bind _pipepath_2 (Variables|Default|GetPipePath))
  (bind _pipepath_3 (Variables|Default|GetPipePath))
  (Utilities|FlowControl|Sequence
    (:then_0
      (LocalVariables|SetLocal_Num_Spline%20_Points (Spline|GetNumberOfSplinePoints (Variables|Default|GetPipePath)))
      (LocalVariables|SetLocal_Spline_World_Transform (Transformation|GetWorldTransform (Variables|Default|GetPipePath))))
    (:then_1
      (for _index (range 0 (LocalVariables|GetLocal_Num_Spline%20_Points))
        (Math|Integer|CompareInt (Utilities|Array|Length _pipe_data) (LocalVariables|GetLocal_Num_Spline%20_Points) :!label _label
          (:>
            (Utilities|Array|RemoveIndex _pipe_data (Utilities|Array|LastIndex _pipe_data))
            (goto _label))
          (:<
            (Utilities|Array|Add :TargetArray _pipe_data)
            (goto _label)))))
    (:then_2
      (for _index_2 (range 0 (- (LocalVariables|GetLocal_Num_Spline%20_Points) 1))
        (LocalVariables|SetLocal_Current_Joint_Index _index_2)
        (if (.addjoint (Utilities|Array|Get(acopy) (Variables|Default|GetPipe_Data) (LocalVariables|GetLocal_Current_Joint_Index)))
          (bind _returnvalue (AddComponent|AddStaticMeshComponent false))
          (Components|StaticMesh|SetStaticMesh _returnvalue (Variables|Default|GetJoint%20Element))
          (Transformation|SetWorldTransform _returnvalue (Math|Transform|ComposeTransforms (Math|Transform|MakeTransform "0, 0, 0" (Math|Rotator|MakeRotator (.rotatejoint (Utilities|Array|Get(acopy) (Variables|Default|GetPipe_Data) (LocalVariables|GetLocal_Current_Joint_Index))) 0.0 0.0)) (Spline|GetTransformatSplinePoint (Variables|Default|GetPipePath) (LocalVariables|GetLocal_Current_Joint_Index) "World" false)) false false))))
    (:then_3
      (for _index_3 (range 0 (- (LocalVariables|GetLocal_Num_Spline%20_Points) 2))
        (LocalVariables|SetLocal_Current_Spine_Index _index_3)
        (bind _returnvalue_2 (AddComponent|AddSplineMeshComponent false))
        (bind _output_get (LocalVariables|SetLocal_Current_Spline_Mesh _returnvalue_2))
        (Components|StaticMesh|SetStaticMesh _output_get (Variables|Default|GetPipe%20Element))
        (SplineMesh|SetStartandEnd _output_get (.Location (Spline|GetLocationandTangentatSplinePoint _pipepath (LocalVariables|GetLocal_Current_Spine_Index) "Local")) (.Tangent (Spline|GetLocationandTangentatSplinePoint _pipepath (LocalVariables|GetLocal_Current_Spine_Index) "Local")) (.Location (Spline|GetLocationandTangentatSplinePoint _pipepath (+ (LocalVariables|GetLocal_Current_Spine_Index) 1) "Local")) (.Tangent (Spline|GetLocationandTangentatSplinePoint _pipepath (+ (LocalVariables|GetLocal_Current_Spine_Index) 1) "Local")) true :!class /Script/Engine.SplineMeshComponent)))
    (:then_4
      (for _index_4 (range 0 (- (Utilities|Array|Length (Variables|Default|GetAddObject_Data)) 1))
        (LocalVariables|SetLocal_Current_AddActorIndex _index_4)
        (Utilities|IsValid (.actor (Utilities|Array|Get(acopy) (Variables|Default|GetAddObject_Data) (LocalVariables|GetLocal_Current_AddActorIndex)))
          (:Is%20Valid
            (bind _returnvalue_3 (AddComponent|AddStaticMeshComponent false))
            (Components|StaticMesh|SetStaticMesh _returnvalue_3 (.actor (Utilities|Array|Get(acopy) (Variables|Default|GetAddObject_Data) (LocalVariables|GetLocal_Current_AddActorIndex))))
            (Transformation|SetWorldTransform _returnvalue_3 (Math|Transform|ComposeTransforms (Math|Transform|MakeTransform "0, 0, 0" (Math|Rotator|MakeRotator (.X (Math|Vector|BreakVector (.offsetrotation (Utilities|Array|Get(acopy) (Variables|Default|GetAddObject_Data) (LocalVariables|GetLocal_Current_AddActorIndex))))) (.Y (Math|Vector|BreakVector (.offsetrotation (Utilities|Array|Get(acopy) (Variables|Default|GetAddObject_Data) (LocalVariables|GetLocal_Current_AddActorIndex))))) (.Z (Math|Vector|BreakVector (.offsetrotation (Utilities|Array|Get(acopy) (Variables|Default|GetAddObject_Data) (LocalVariables|GetLocal_Current_AddActorIndex)))))) (.scale (Utilities|Array|Get(acopy) (Variables|Default|GetAddObject_Data) (LocalVariables|GetLocal_Current_AddActorIndex)))) (Math|Transform|MakeTransform (Spline|GetLocationatDistanceAlongSpline _pipepath_3 (* (Spline|GetSplineLength (Variables|Default|GetPipePath)) (.percentoncurve (Utilities|Array|Get(acopy) (Variables|Default|GetAddObject_Data) (LocalVariables|GetLocal_Current_AddActorIndex)))) "World") (Math|Conversions|RotationFromXVector (- (Spline|GetLocationatDistanceAlongSpline _pipepath_3 (+ (* (Spline|GetSplineLength (Variables|Default|GetPipePath)) (.percentoncurve (Utilities|Array|Get(acopy) (Variables|Default|GetAddObject_Data) (LocalVariables|GetLocal_Current_AddActorIndex)))) 0.01) "World") (Spline|GetLocationatDistanceAlongSpline _pipepath_3 (* (Spline|GetSplineLength (Variables|Default|GetPipePath)) (.percentoncurve (Utilities|Array|Get(acopy) (Variables|Default|GetAddObject_Data) (LocalVariables|GetLocal_Current_AddActorIndex)))) "World"))))) false false)))))
    (:then_5
      (if (Variables|Default|GetDraw%20Spline%20Indicies)
        (for _index_5 (range 0 (- (Spline|GetNumberOfSplinePoints _pipepath_2) 1))
          (bind _returnvalue_4 (AddComponent|AddTextRenderComponent false (Math|Transform|MakeTransform (+ (.Location (Spline|GetLocationandTangentatSplinePoint _pipepath_2 _index_5 "Local")) (* (Class|SplineComponent|GetUpVectoratSplinePoint _pipepath_2 _index_5 "Local") (Variables|Default|GetIndicies%20Offset))) (Math|Conversions|RotationFromXVector (* (.Tangent (Spline|GetLocationandTangentatSplinePoint _pipepath_2 _index_5 "Local")) -1.0)))))
          (Rendering|Components|TextRender|SetText _returnvalue_4 (Utilities|Text|ToText(Integer) _index_5)))))))