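; Procedural ivy generator that scatters instanced leaf meshes over nearby surfaces, built entirely in the Construction Script.
; CastSphere sphere-traces forward, then steps each successful cast upward with random horizontal variation, optionally adding debug spheres and arrows.
; Each hit records an impact point and adds randomly offset leaves.
; Surface wrapping looks unfinished: misses rotate NewStart, whose creation never runs, WrapCasting is a stub, and seeded randomness is unused.
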(event EventBeginPlay)

(event Collision|EventActorBeginOverlap
  (params (OtherActor :type Actor%20Object%20Reference)))

(event EventTick
  (params (DeltaSeconds :type Float%20%28single-precision%29)))

(fn ConstructionScript
  (bind _hitpoints (Variables|Default|GetHitPoints))
  (bind _lastimpactpoint (Variables|Default|GetLastImpactPoint))
  (bind _defaultsceneroot (Variables|Default|GetDefaultSceneRoot))
  (bind _newstart (Variables|Default|GetNewStart))
  (bind _impactpoint (Variables|Default|GetImpactPoint))
  (bind _leaf_spacing (Variables|Default|GetLeaf%20Spacing))
  (bind _returnvalue (* _leaf_spacing -1.0))
  (bind _output_get (Variables|Default|SetCast%20Start (Transformation|GetWorldLocation _defaultsceneroot)))
  (Variables|Default|SetCast%20End (+ _output_get (* (Math|Vector|GetForwardVector _defaultsceneroot) (Variables|Default|GetTrace%20Distance))))
  (while (not (Variables|Default|GetStopCasting))
    (bind _index (Utilities|FlowControl|ForLoopwithBreak 0 (- (Variables|Default|GetCastPoint%20Count) 1))
      (:LoopBody
        (if (LocalVariables|GetNotFirst)
          _
          (else
            (LocalVariables|SetNotFirst true)))
        (Variables|Default|SetCastPointIndex _index)
        (if (not (Variables|Default|GetStopCasting))
          (Variables|Default|SetHit%20Attempt 1)
          (bind (_gothit _impactpoint_2 _spherelocation) (CallFunction|CastSphere (Variables|Default|GetCast%20Start) (Variables|Default|GetCast%20End) (Variables|Default|GetTrace%20Radius)))
          (if _gothit
            (bind _output_get_2 (LocalVariables|SetHitSphereLocation _spherelocation))
            (Math|Integer|IncrementInt _hitpoints
              (:%20%20
                (Utilities|Array|SetArrayElem _impactpoint (- _hitpoints 1) _lastimpactpoint true)
                (for _index_2 (range 0 (- (Variables|Default|GetLeaves) 1))
                  (Components|InstancedStaticMesh|AddInstance (Variables|Default|GetInstancedStaticMesh) (Math|Transform|MakeTransform (Math|Vector|MakeVector (.X (Math|Vector|BreakVector (.location (Math|Transform|MakeRelativeTransform (Math|Transform|MakeTransform (Utilities|Array|Get(acopy) _impactpoint _hitpoints) (Math|Rotator|FindLookatRotation _lastimpactpoint _output_get_2) "2.000000,2.000000,2.000000") (Transformation|GetRelativeTransform (Variables|Default|GetDefaultSceneRoot)))))) (+ (.Y (Math|Vector|BreakVector (.location (Math|Transform|MakeRelativeTransform (Math|Transform|MakeTransform (Utilities|Array|Get(acopy) _impactpoint _hitpoints) (Math|Rotator|FindLookatRotation _lastimpactpoint _output_get_2) "2.000000,2.000000,2.000000") (Transformation|GetRelativeTransform (Variables|Default|GetDefaultSceneRoot)))))) (Math|Random|RandomFloatinRange _returnvalue _leaf_spacing)) (+ (.Z (Math|Vector|BreakVector (.location (Math|Transform|MakeRelativeTransform (Math|Transform|MakeTransform (Utilities|Array|Get(acopy) _impactpoint _hitpoints) (Math|Rotator|FindLookatRotation _lastimpactpoint _output_get_2) "2.000000,2.000000,2.000000") (Transformation|GetRelativeTransform (Variables|Default|GetDefaultSceneRoot)))))) (Math|Random|RandomFloatinRange _returnvalue _leaf_spacing))) (Variables|Default|GetLeaf%20Rotation) (.scale (Math|Transform|MakeRelativeTransform (Math|Transform|MakeTransform (Utilities|Array|Get(acopy) _impactpoint _hitpoints) (Math|Rotator|FindLookatRotation _lastimpactpoint _output_get_2) "2.000000,2.000000,2.000000") (Transformation|GetRelativeTransform (Variables|Default|GetDefaultSceneRoot)))))))))
            (else
              (bind _result (Math|Integer|IncrementInt (Variables|Default|GetHit%20Attempt))
                (:%20%20
                  (Variables|Default|SetHit%20Attempt _result)
                  (Variables|Default|SetStopCasting (>= (Variables|Default|GetHit%20Attempt) (Variables|Default|GetMax%20Attempts)))
                  (Transformation|AddWorldRotation _newstart (Math|Rotator|FindLookatRotation (Transformation|GetWorldLocation _newstart) (Utilities|Array|Get(acopy) (Variables|Default|GetImpactPoint) (- (Variables|Default|GetCastPointIndex) 1))) false false)))))))
      (:Completed
        (Utilities|Array|Resize (Variables|Default|GetImpactPoint) (Variables|Default|GetHitPoints))
        (Variables|Default|SetStopCasting true))))
  (Utilities|FlowControl|ForLoopwithBreak 0 (- (Variables|Default|GetCastPoint%20Count) 1)) ; enters at Break
)

(fn CastSphere
  (params (Start :type Vector) (End :type Vector) (Radius :type Float%20%28single-precision%29))
  (bind _defaultsceneroot (Variables|Default|GetDefaultSceneRoot))
  (bind _horizontal_variation (Variables|Default|GetHorizontal%20Variation))
  (bind _castpoint_spacing (Variables|Default|GetCastPoint%20Spacing))
  (bind _returnvalue (Math|Vector|GetUpVector _defaultsceneroot))
  (bind _returnvalue_2 (* _returnvalue _castpoint_spacing))
  (bind (_outhit _returnvalue_3) (Collision|SphereTraceForObjects Start End Radius (Variables|Default|GetObject%20Type%20Array) false 0 "None" true "(R=1.000000,G=0.000000,B=0.000000,A=1.000000)" "(R=0.000000,G=1.000000,B=0.000000,A=1.000000)" 1.0))
  (if _returnvalue_3
    (Variables|Default|SetLastImpactPoint (.impactpoint _outhit))
    (bind _output_get (LocalVariables|SetHitSphereLocation (.location _outhit)))
    (LocalVariables|SetHitPoint (.impactpoint _outhit))
    (if (Variables|Default|GetVisualizeCasting)
      (AddComponent|AddSphereComponent false (Math|Transform|MakeTransform (.location (Math|Transform|MakeRelativeTransform (Math|Conversions|ToTransform(Vector) _output_get) (Transformation|GetActorTransform))) (.rotation (Math|Transform|MakeRelativeTransform (Math|Conversions|ToTransform(Vector) _output_get) (Transformation|GetActorTransform))) (* (.scale (Math|Transform|MakeRelativeTransform (Math|Conversions|ToTransform(Vector) _output_get) (Transformation|GetActorTransform))) (/ (Variables|Default|GetTrace%20Radius) 33.0))))
      (AddComponent|AddArrowComponent false (Math|Transform|MakeRelativeTransform (Math|Transform|MakeTransform (Variables|Default|GetCast%20Start) (Math|Rotator|FindLookatRotation (Variables|Default|GetCast%20Start) (LocalVariables|GetHitPoint))) (Transformation|GetActorTransform)))
      (AddComponent|AddArrowComponent false (Math|Transform|MakeRelativeTransform (Math|Transform|MakeTransform (LocalVariables|GetHitPoint) (Math|Rotator|FindLookatRotation (LocalVariables|GetHitPoint) (LocalVariables|GetHitSphereLocation))) (Transformation|GetActorTransform))))
    (Variables|Default|SetCast%20Start (Math|Vector|MakeVector (.x (+ (Variables|Default|GetCast%20Start) _returnvalue_2)) (+ (.y (+ (Variables|Default|GetCast%20Start) _returnvalue_2)) (Math|Random|RandomFloatinRange _horizontal_variation (* _horizontal_variation -1.0))) (.z (+ (Variables|Default|GetCast%20Start) _returnvalue_2))))
    (Variables|Default|SetCast%20End (Math|Vector|MakeVector (.x (+ _returnvalue_2 (Variables|Default|GetCast%20End))) (+ (.y (+ (Variables|Default|GetCast%20Start) _returnvalue_2)) (Math|Random|RandomFloatinRange _horizontal_variation (* _horizontal_variation -1.0))) (.z (+ _returnvalue_2 (Variables|Default|GetCast%20End))))))
  (return _returnvalue_3 (LocalVariables|GetHitPoint) (LocalVariables|GetHitSphereLocation)))

(fn WrapCasting
  (return "0, 0, 0" "0, 0, 0"))