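; Construction-script Blueprint that builds a road or track along a spline, either looping or open.
; It resizes a per-point data array to match the spline points, then spawns spline mesh segments for the road and optional left and right guard rails.
; Each point's data sets bank, width and height scaling, and mesh overrides, with segments interpolating to the next point.
; An optional debug mode labels each spline point with its index.
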(event EventBeginPlay)

(event Collision|EventActorBeginOverlap
  (params (OtherActor :type Actor%20Object%20Reference)))

(event EventTick
  (params (DeltaSeconds :type Float%20%28single-precision%29)))

(fn ConstructionScript
  (bind _spline (Variables|Components|GetSpline))
  (Utilities|FlowControl|Sequence
    (:then_0
      (|NumberSplinePoints))
    (:then_1
      (|BuildRoadDataArray))
    (:then_2
      (for _index (range 0 (- (Variables|Default|GetNumber%20Of%20Spline%20Points) (Math|Integer|SelectInt 1 2 (Variables|TrackSetup|GetLooping%20Track))))
        (LocalVariables|SetLocal_LoopIndex _index)
        (Utilities|FlowControl|Sequence
          (:then_0
            (CallFunction|BuildTrackElement (LocalVariables|GetLocal_LoopIndex) (Variables|DefaultTrackElements|GetRoadMesh) (.customelement (Utilities|Array|Get(acopy) (Variables|TrackSetup|GetRoad%20Data%20Array) (LocalVariables|GetLocal_LoopIndex)))))
          (:then_1
            (if (.leftguardrail (Utilities|Array|Get(acopy) (Variables|TrackSetup|GetRoad%20Data%20Array) (LocalVariables|GetLocal_LoopIndex)))
              (CallFunction|BuildTrackElement (LocalVariables|GetLocal_LoopIndex) (Variables|DefaultTrackElements|GetLeftRailMesh) (.customleftrailing (Utilities|Array|Get(acopy) (Variables|TrackSetup|GetRoad%20Data%20Array) (LocalVariables|GetLocal_LoopIndex))))))
          (:then_2
            (if (.rightguardrail (Utilities|Array|Get(acopy) (Variables|TrackSetup|GetRoad%20Data%20Array) (LocalVariables|GetLocal_LoopIndex)))
              (CallFunction|BuildTrackElement (LocalVariables|GetLocal_LoopIndex) (Variables|DefaultTrackElements|GetRightRailMesh) (.customrightrailing (Utilities|Array|Get(acopy) (Variables|TrackSetup|GetRoad%20Data%20Array) (LocalVariables|GetLocal_LoopIndex)))))))))
    (:then_3
      (if (Variables|TrackSetup|GetDraw%20Track%20Points)
        (for _index_2 (range 0 (- (Spline|GetNumberOfSplinePoints _spline) 1))
          (bind _returnvalue (AddComponent|AddTextRenderComponent false (Math|Transform|MakeTransform (Math|Vector|MakeVector (.X (Math|Vector|BreakVector (.Location (Spline|GetLocationandTangentatSplinePoint _spline _index_2 "Local")))) (.Y (Math|Vector|BreakVector (.Location (Spline|GetLocationandTangentatSplinePoint _spline _index_2 "Local")))) (+ (.Z (Math|Vector|BreakVector (.Location (Spline|GetLocationandTangentatSplinePoint _spline _index_2 "Local")))) 5e+01)) (Math|Conversions|RotationFromXVector (* (.Tangent (Spline|GetLocationandTangentatSplinePoint _spline _index_2 "Local")) -1.0)))))
          (Rendering|Components|TextRender|SetText _returnvalue (Utilities|Text|ToText(Integer) _index_2)))))))

(fn BuildTrackElement
  (params (Loop%20Index :type Integer) (Track%20Element%20Mesh :type Static%20Mesh%20Object%20Reference) (Track%20Element%20Override :type Static%20Mesh%20Object%20Reference))
  (LocalVariables|SetLocal_CurrentLoopIndex Loop%20Index)
  (LocalVariables|SetLocal_NextLoopIndex (Math|Integer|%(Integer) (+ Loop%20Index 1) (Variables|Default|GetNumber%20Of%20Spline%20Points)))
  (LocalVariables|SetLocal_TrackEleMesh Track%20Element%20Mesh)
  (LocalVariables|SetLocal_ElementOverrideMesh Track%20Element%20Override)
  (Utilities|FlowControl|Sequence
    (:then_0
      (LocalVariables|SetLocal_StartLocation (.Location (Spline|GetLocationandTangentatSplinePoint (Variables|Components|GetSpline) (LocalVariables|GetLocal_CurrentLoopIndex) "Local")))
      (LocalVariables|SetLocal_StartTan (.Tangent (Spline|GetLocationandTangentatSplinePoint (Variables|Components|GetSpline) (LocalVariables|GetLocal_CurrentLoopIndex) "Local")))
      (LocalVariables|SetLocal_EndLocation (.Location (Spline|GetLocationandTangentatSplinePoint (Variables|Components|GetSpline) (LocalVariables|GetLocal_NextLoopIndex) "Local")))
      (LocalVariables|SetLocal_EndTan (.Tangent (Spline|GetLocationandTangentatSplinePoint (Variables|Components|GetSpline) (LocalVariables|GetLocal_NextLoopIndex) "Local")))
      (LocalVariables|SetLocal_StartRoll (.bank (Utilities|Array|Get(acopy) (Variables|TrackSetup|GetRoad%20Data%20Array) (LocalVariables|GetLocal_CurrentLoopIndex))))
      (LocalVariables|SetLocal_StartScale (Math|Vector2D|MakeVector2D (* (Variables|TrackSetup|GetWidth) (.width (Utilities|Array|Get(acopy) (Variables|TrackSetup|GetRoad%20Data%20Array) (LocalVariables|GetLocal_CurrentLoopIndex)))) (* (Variables|TrackSetup|GetHeight) (.height (Utilities|Array|Get(acopy) (Variables|TrackSetup|GetRoad%20Data%20Array) (LocalVariables|GetLocal_CurrentLoopIndex))))))
      (LocalVariables|SetLocal_EndRoll (.bank (Utilities|Array|Get(acopy) (Variables|TrackSetup|GetRoad%20Data%20Array) (LocalVariables|GetLocal_NextLoopIndex))))
      (LocalVariables|SetLocal_EndScale (Math|Vector2D|MakeVector2D (* (Variables|TrackSetup|GetWidth) (.width (Utilities|Array|Get(acopy) (Variables|TrackSetup|GetRoad%20Data%20Array) (LocalVariables|GetLocal_NextLoopIndex)))) (* (Variables|TrackSetup|GetHeight) (.height (Utilities|Array|Get(acopy) (Variables|TrackSetup|GetRoad%20Data%20Array) (LocalVariables|GetLocal_NextLoopIndex)))))))
    (:then_1
      (bind _returnvalue (AddComponent|AddSplineMeshComponent false))
      (LocalVariables|SetLocal_CurrentSplineMesh _returnvalue)
      (Utilities|IsValid (LocalVariables|GetLocal_ElementOverrideMesh)
        (:Is%20Valid
          (Components|StaticMesh|SetStaticMesh (LocalVariables|GetLocal_CurrentSplineMesh) (LocalVariables|GetLocal_ElementOverrideMesh)))
        (:Is%20Not%20Valid
          (Components|StaticMesh|SetStaticMesh (LocalVariables|GetLocal_CurrentSplineMesh) (LocalVariables|GetLocal_TrackEleMesh))))
      (SplineMesh|SetStartandEnd (LocalVariables|GetLocal_CurrentSplineMesh) (LocalVariables|GetLocal_StartLocation) (LocalVariables|GetLocal_StartTan) (LocalVariables|GetLocal_EndLocation) (LocalVariables|GetLocal_EndTan) true :!class /Script/Engine.SplineMeshComponent)
      (Class|SplineMeshComponent|SetStartRoll (LocalVariables|GetLocal_CurrentSplineMesh) (Math|Trig|DegreesToRadians (LocalVariables|GetLocal_StartRoll)) true)
      (Class|SplineMeshComponent|SetEndRoll (LocalVariables|GetLocal_CurrentSplineMesh) (Math|Trig|DegreesToRadians (LocalVariables|GetLocal_EndRoll)) true)
      (SplineMesh|SetStartScale (LocalVariables|GetLocal_CurrentSplineMesh) (LocalVariables|GetLocal_StartScale) true :!class /Script/Engine.SplineMeshComponent)
      (SplineMesh|SetEndScale (LocalVariables|GetLocal_CurrentSplineMesh) (LocalVariables|GetLocal_EndScale) true :!class /Script/Engine.SplineMeshComponent)
      (Collision|SetCollisionEnabled (LocalVariables|GetLocal_CurrentSplineMesh) (select (Variables|TrackSetup|GetCollisions%20Enabled) "QueryAndPhysics" "NoCollision")))))