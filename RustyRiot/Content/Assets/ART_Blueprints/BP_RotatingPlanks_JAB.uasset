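; BP_RotatingPlanks_JAB is a construction-script tool that places copies of a chosen mesh, such as planks, at regular spacing along a spline.
; Each copy is an unattached static mesh component at the spline's world position, with a shared scale, material and roll.
; A random stream varies each pitch within a set range; spline direction is ignored and nothing rotates at runtime.
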(event EventBeginPlay)

(event Collision|EventActorBeginOverlap
  (params (OtherActor :type Actor%20Object%20Reference)))

(event EventTick
  (params (DeltaSeconds :type Float%20%28single-precision%29)))

(fn ConstructionScript
  (bind _splinecomponentexample (Variables|Default|GetSplineComponentExample))
  (bind _spacing (Variables|Mesh|Getspacing))
  (for _index (range 1 (.ReturnValue (Math|Float|Division(WholeandRemainder) (Spline|GetSplineLength _splinecomponentexample) _spacing)))
    (bind _returnvalue (AddComponent|AddStaticMeshComponent true (Math|Transform|MakeTransform (Spline|GetLocationatDistanceAlongSpline _splinecomponentexample (* (Math|Conversions|ToFloat(Integer) _index) _spacing) "World") (Math|Rotator|MakeRotator (Variables|Mesh|GetVertical%20Rotation) (Math|Random|RandomFloatinRangefromStream (Variables|Mesh|GetMin%20Rotate) (Variables|Mesh|GetMax%20Rotate) (Variables|Default|GetRandomStream)) 0.0) (Math|Vector|MakeVector (Variables|Mesh|GetScale%20X) (Variables|Mesh|GetScale%20Y) (Variables|Mesh|GetScale%20Z)))))
    (Components|StaticMesh|SetStaticMesh _returnvalue (Variables|Mesh|GetType%20of%20Mesh))
    (Rendering|Material|SetMaterial _returnvalue 0 (Variables|Mesh|GetMaterial))))