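; BP_DestructibleMesh_JAB is a Blueprint wrapper that places a configurable destructible mesh with a cull distance.
; The construction script adds a Destructible component, assigns the Mesh variable to it, applies CullDistance and resets SpriteScale to 1.
; Event Tick reapplies the same cull distance to the component every frame.
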(event EventTick
  (params (DeltaSeconds :type Float%20%28single-precision%29))
  (Class|PrimitiveComponent|SetCullDistance (Variables|Default|GetDestructible) (Variables|Default|GetCull%20Distance)))

(fn ConstructionScript
  (Utilities|FlowControl|Sequence
    (:then_0
      (AddComponent|AddDestructibleComponent false)
      (Class|DestructibleComponent|SetDestructibleMesh (Variables|Default|GetDestructible) (Variables|Default|GetMesh))
      (Class|PrimitiveComponent|SetCullDistance (Variables|Default|GetDestructible) (Variables|Default|GetCull%20Distance)))
    (:then_1
      (Variables|Default|SetSpriteScale 1.0))))