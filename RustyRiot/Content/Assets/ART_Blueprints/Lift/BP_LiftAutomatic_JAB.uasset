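; Automatic lift that rides between bottom and top when its trigger box is overlapped, picking direction from AtBottom.
; One timeline moves ElevatorRoot vertically and updates AtBottom on finish, while another pitches the two lift doors in parallel.
; The overlap also signals every BP_LiftFloorDoor_JAB in the level.
; Lift_Up and Lift_Down events provide delayed lever commands that run the same timelines without signalling floor doors.
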(event OnComponentBeginOverlap(Box_Trigger)
  (params (OverlappedComponent :type Primitive%20Component%20Object%20Reference) (OtherActor :type Actor%20Object%20Reference) (OtherComp :type Primitive%20Component%20Object%20Reference) (OtherBodyIndex :type Integer) (bFromSweep :type Boolean) (SweepResult :type Hit%20Result%20Structure%20%28by%20ref%29))
  ;[1 1 1] Overlay for Inputs
  (if (Variables|Default|GetAtBottom)
    (Utilities|FlowControl|Sequence
      (:then_0
        ;[1 1 1] Send Command to Floor Doors
        (bind _outactors (Actor|GetAllActorsOfClass "/Game/Assets/ART_Blueprints/Lift/BP_LiftFloorDoor_JAB.BP_LiftFloorDoor_JAB_C"))
        (for _array_element _outactors
          (Default|LiftUpAuto _array_element)))
      (:then_1
        ;[1 1 1] Lift Up & Down
        (bind (_direction _elevator_up) (Timeline|Lift%20Up%20Down Play)
          (:Update
            (Transformation|SetRelativeLocation (Variables|Default|GetElevator_Root) (Math|Vector|MakeVector 0.0 0.0 (* _elevator_up (Variables|Default|GetElevator%20Max%20Height))) false false))
          (:Finished
            (if (Utilities|Enum|Equal(Enum) _direction "Forward")
              (Variables|Default|SetAtBottom false)
              (else
                (Variables|Default|SetAtBottom true))))))
      (:then_2
        ;[1 1 1] Lift Doors
        (bind _doors_up_down (Timeline|Doors Play)
          (:Update
            (Transformation|SetRelativeRotation (Variables|Default|GetSM_LiftDoor_01_JAB) (Math|Rotator|MakeRotator 0.0 (* _doors_up_down (Variables|Default|GetMaxRotationDoor1)) 0.0) false false)
            (Transformation|SetRelativeRotation (Variables|Default|GetSM_LiftDoor_02_JAB) (Math|Rotator|MakeRotator 0.0 (* _doors_up_down (Variables|Default|GetMaxRotationDoor2)) 0.0) false false)))))
    (else
      (Utilities|FlowControl|Sequence
        (:then_0
          (bind _outactors_2 (Actor|GetAllActorsOfClass "/Game/Assets/ART_Blueprints/Lift/BP_LiftFloorDoor_JAB.BP_LiftFloorDoor_JAB_C"))
          (for _array_element_2 _outactors_2
            (Default|LiftDownAuto _array_element_2)))
        (:then_1
          (Timeline|Lift%20Up%20Down Reverse))
        (:then_2
          (Timeline|Doors Reverse))))))

(event Custom|Lift_Up
  ;[1 1 1] Lever Commands with Delay
  (Utilities|FlowControl|Delay (Variables|Default|GetDelay))
  (Utilities|FlowControl|Sequence
    (:then_0
      ;[1 1 1] Lift Doors
      (bind _doors_up_down (Timeline|Doors Play)
        (:Update
          (Transformation|SetRelativeRotation (Variables|Default|GetSM_LiftDoor_01_JAB) (Math|Rotator|MakeRotator 0.0 (* _doors_up_down (Variables|Default|GetMaxRotationDoor1)) 0.0) false false)
          (Transformation|SetRelativeRotation (Variables|Default|GetSM_LiftDoor_02_JAB) (Math|Rotator|MakeRotator 0.0 (* _doors_up_down (Variables|Default|GetMaxRotationDoor2)) 0.0) false false))))
    (:then_1
      ;[1 1 1] Lift Up & Down
      (bind (_direction _elevator_up) (Timeline|Lift%20Up%20Down Play)
        (:Update
          (Transformation|SetRelativeLocation (Variables|Default|GetElevator_Root) (Math|Vector|MakeVector 0.0 0.0 (* _elevator_up (Variables|Default|GetElevator%20Max%20Height))) false false))
        (:Finished
          (if (Utilities|Enum|Equal(Enum) _direction "Forward")
            (Variables|Default|SetAtBottom false)
            (else
              (Variables|Default|SetAtBottom true))))))))

(event Custom|Lift_Down
  ;[1 1 1] Lever Commands with Delay
  (Utilities|FlowControl|Delay (Variables|Default|GetDelay))
  (Utilities|FlowControl|Sequence
    (:then_0
      ;[1 1 1] Lift Up & Down
      (bind (_direction _elevator_up) (Timeline|Lift%20Up%20Down Reverse)
        (:Update
          (Transformation|SetRelativeLocation (Variables|Default|GetElevator_Root) (Math|Vector|MakeVector 0.0 0.0 (* _elevator_up (Variables|Default|GetElevator%20Max%20Height))) false false))
        (:Finished
          (if (Utilities|Enum|Equal(Enum) _direction "Forward")
            (Variables|Default|SetAtBottom false)
            (else
              (Variables|Default|SetAtBottom true))))))
    (:then_1
      ;[1 1 1] Lift Doors
      (bind _doors_up_down (Timeline|Doors Reverse)
        (:Update
          (Transformation|SetRelativeRotation (Variables|Default|GetSM_LiftDoor_01_JAB) (Math|Rotator|MakeRotator 0.0 (* _doors_up_down (Variables|Default|GetMaxRotationDoor1)) 0.0) false false)
          (Transformation|SetRelativeRotation (Variables|Default|GetSM_LiftDoor_02_JAB) (Math|Rotator|MakeRotator 0.0 (* _doors_up_down (Variables|Default|GetMaxRotationDoor2)) 0.0) false false))))))

(fn ConstructionScript)