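; Lift floor door Blueprint that rotates a door open and closed as the lift moves up or down.
; The OpenCloseDoor timeline scales DoorMaxRotation to set the door's relative roll, playing forward on up commands and reversing on down commands.
; Lever-triggered events wait for a configurable delay, while the Auto events from the lift itself act immediately.
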(event Custom|Lift_Up_Auto
  ;[1 1 1] Door Commands from Lift No Delay
  (bind _open_door (Timeline|Open/Close%20Door Play)
    (:Update
      (Transformation|SetRelativeRotation (Variables|Default|GetLift_Floor_Door) (Math|Rotator|MakeRotator (* _open_door (Variables|Default|GetDoor%20Max%20Rotation)) 0.0 0.0) false false))))

(event Custom|Lift_Down_Auto
  ;[1 1 1] Door Commands from Lift No Delay
  (bind _open_door (Timeline|Open/Close%20Door Reverse)
    (:Update
      (Transformation|SetRelativeRotation (Variables|Default|GetLift_Floor_Door) (Math|Rotator|MakeRotator (* _open_door (Variables|Default|GetDoor%20Max%20Rotation)) 0.0 0.0) false false))))

(event Custom|Lift_Up
  ;[1 1 1] Door Commands from Lever with Delay
  (Utilities|FlowControl|Delay (Variables|Default|GetDelay))
  (bind _open_door (Timeline|Open/Close%20Door Play)
    (:Update
      (Transformation|SetRelativeRotation (Variables|Default|GetLift_Floor_Door) (Math|Rotator|MakeRotator (* _open_door (Variables|Default|GetDoor%20Max%20Rotation)) 0.0 0.0) false false))))

(event Custom|Lift_Down
  ;[1 1 1] Door Commands from Lever with Delay
  (Utilities|FlowControl|Delay (Variables|Default|GetDelay))
  (bind _open_door (Timeline|Open/Close%20Door Reverse)
    (:Update
      (Transformation|SetRelativeRotation (Variables|Default|GetLift_Floor_Door) (Math|Rotator|MakeRotator (* _open_door (Variables|Default|GetDoor%20Max%20Rotation)) 0.0 0.0) false false))))

(fn ConstructionScript)