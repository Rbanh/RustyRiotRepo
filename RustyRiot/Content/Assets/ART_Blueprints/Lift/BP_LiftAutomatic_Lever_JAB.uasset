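; Lift control lever that lets the player send a lift up with E or down with Q.
; Overlapping the panel enables input and toggles a help text, which a looping timer keeps turned toward the camera.
; Key presses call the linked LiftButton and every BP_LiftFloorDoor_JAB actor in the level, while a timeline plays or reverses to tilt the lever stick.
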(event OnComponentBeginOverlap(Panel)
  (params (OverlappedComponent :type Primitive%20Component%20Object%20Reference) (OtherActor :type Actor%20Object%20Reference) (OtherComp :type Primitive%20Component%20Object%20Reference) (OtherBodyIndex :type Integer) (bFromSweep :type Boolean) (SweepResult :type Hit%20Result%20Structure%20%28by%20ref%29))
  ;[1 1 1] Overlay for Input
  (Utilities|FlowControl|Sequence
    (:then_0
      (Utilities|Casting|CastTo OtherActor))
    (:then_1
      (Utilities|Casting|CastTo OtherActor))
    (:then_2
      (Utilities|Casting|CastTo OtherActor)))
  (Input|EnableInput (Game|GetPlayerController 0))
  ;[1 1 1] Helpfull Text
  (Rendering|ToggleVisibility (Variables|Default|GetHelpful%20Text) false))

(event OnComponentEndOverlap(Panel)
  (params (OverlappedComponent :type Primitive%20Component%20Object%20Reference) (OtherActor :type Actor%20Object%20Reference) (OtherComp :type Primitive%20Component%20Object%20Reference) (OtherBodyIndex :type Integer))
  ;[1 1 1] Overlay for Input
  (Utilities|FlowControl|Sequence
    (:then_0
      (Utilities|Casting|CastTo OtherActor))
    (:then_1
      (Utilities|Casting|CastTo OtherActor))
    (:then_2
      (Utilities|Casting|CastTo OtherActor)))
  (Input|DisableInput (Game|GetPlayerController 0))
  ;[1 1 1] Helpfull Text
  (Rendering|ToggleVisibility (Variables|Default|GetHelpful%20Text) false))

(event EventBeginPlay
  ;[1 1 1] Helpfull Text
  (Utilities|Time|SetTimerbyFunctionName 0 "GetAngle" 0.1 true))

(event Input|KeyboardEvents|E
  (params (Key :type Key%20Structure))
  ;[1 1 1] Lever Rotation
  (:Pressed
    (bind _leverrotation (Timeline|Lever_Rotation Play)
      (:Update
        (Transformation|SetRelativeRotation (Variables|Default|GetSM_LeverStick_JAB) (Math|Rotator|MakeRotator 0.0 (* _leverrotation (Variables|Default|GetLeverRotation)) 0.0) false false)))))

(event Input|KeyboardEvents|Q
  (params (Key :type Key%20Structure))
  ;[1 1 1] Lever Rotation
  (:Pressed
    (bind _leverrotation (Timeline|Lever_Rotation Reverse)
      (:Update
        (Transformation|SetRelativeRotation (Variables|Default|GetSM_LeverStick_JAB) (Math|Rotator|MakeRotator 0.0 (* _leverrotation (Variables|Default|GetLeverRotation)) 0.0) false false)))))

(event Input|KeyboardEvents|Q
  (params (Key :type Key%20Structure))
  ;[1 1 1] Keyboard Commands Doors
  (:Pressed
    (bind _outactors (Actor|GetAllActorsOfClass "/Game/Assets/ART_Blueprints/Lift/BP_LiftFloorDoor_JAB.BP_LiftFloorDoor_JAB_C"))
    (for _array_element _outactors
      (Default|LiftDown _array_element))))

(event Input|KeyboardEvents|E
  (params (Key :type Key%20Structure))
  ;[1 1 1] Keyboard Commands Doors
  (:Pressed
    (bind _outactors (Actor|GetAllActorsOfClass "/Game/Assets/ART_Blueprints/Lift/BP_LiftFloorDoor_JAB.BP_LiftFloorDoor_JAB_C"))
    (for _array_element _outactors
      (Default|LiftUp _array_element))))

(event Input|KeyboardEvents|E
  (params (Key :type Key%20Structure))
  ;[1 1 1] Keyboard Commands Lift
  (:Pressed
    (Default|LiftUp (Variables|Default|GetLift_Button))))

(event Input|KeyboardEvents|Q
  (params (Key :type Key%20Structure))
  ;[1 1 1] Keyboard Commands Lift
  (:Pressed
    (Default|LiftDown (Variables|Default|GetLift_Button))))

(fn ConstructionScript)

(fn GetAngle
  (Transformation|SetWorldRotation (Variables|Default|GetHelpful%20Text) (Math|Conversions|RotationFromXVector (Math|Vector|Normalize (- (- (Camera|GetCameraLocation (Game|GetPlayerCameraManager 0)) (Transformation|GetActorLocation)) "1.000000,1.000000, 0"))) false false))