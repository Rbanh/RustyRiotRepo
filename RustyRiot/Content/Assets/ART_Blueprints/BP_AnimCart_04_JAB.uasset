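; BP_AnimCart_04_JAB is a destructible cart that travels along a BP_RoadBuilder spline when active.
; A CartMover timeline, scaled by Duration and begun at a start offset, moves a Sphere along the spline's length and rotation.
; Each update looks up every road builder and snaps the Destructible to the Sphere until it breaks.
; A hit or fracture sets Break, detaching the Destructible, and destroys the actor after a delay.
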(event OnComponentFracture(Destructible)
  (params (HitPoint :type Vector%20%28by%20ref%29 :default "0, 0, 0") (HitDirection :type Vector%20%28by%20ref%29 :default "0, 0, 0"))
  ;[1 1 1] Destroy Actor
  (Variables|Default|SetBreak true)
  (Utilities|FlowControl|Delay 1e+01)
  (Actor|DestroyActor))

(event OnComponentHit(Destructible)
  (params (HitComponent :type Primitive%20Component%20Object%20Reference) (OtherActor :type Actor%20Object%20Reference) (OtherComp :type Primitive%20Component%20Object%20Reference) (NormalImpulse :type Vector :default "0, 0, 0") (Hit :type Hit%20Result%20Structure%20%28by%20ref%29))
  ;[1 1 1] Destroy Actor
  (Variables|Default|SetBreak true)
  (Utilities|FlowControl|Delay 1e+01)
  (Actor|DestroyActor))

(event Custom|MoveCart
  (bind _destructible (Variables|Default|GetDestructible))
  (Components|Timeline|SetPlayRate (Variables|Default|GetCartMover) (/ 1.0 (Variables|Default|GetDuration)))
  (Components|Timeline|SetNewTime (Variables|Default|GetCartMover) (Variables|Default|GetCartStartOffSet))
  (bind _alpha (Timeline|CartMover Play)
    (:Update
      (Variables|Default|SetAlpha _alpha)
      (bind _outactors (Actor|GetAllActorsOfClass "/Game/Assets/ART_Blueprints/Paul_BP/BP_RoadBuilder.BP_RoadBuilder_C"))
      (for _array_element _outactors
        (Transformation|SetWorldLocationAndRotation (Variables|Default|GetSphere) (Spline|GetLocationatDistanceAlongSpline (Variables|/Game/Assets/ART_Blueprints/Paul_BP/BP_RoadBuilder.BP_RoadBuilder_C|GetSpline _array_element) (Math|Float|Lerp 0.0 (Spline|GetSplineLength (Variables|/Game/Assets/ART_Blueprints/Paul_BP/BP_RoadBuilder.BP_RoadBuilder_C|GetSpline _array_element)) (Variables|Default|GetAlpha)) "World") (Spline|GetRotationatDistanceAlongSpline (Variables|/Game/Assets/ART_Blueprints/Paul_BP/BP_RoadBuilder.BP_RoadBuilder_C|GetSpline _array_element) (Math|Float|Lerp 0.0 (Spline|GetSplineLength (Variables|/Game/Assets/ART_Blueprints/Paul_BP/BP_RoadBuilder.BP_RoadBuilder_C|GetSpline _array_element)) (Variables|Default|GetAlpha)) "World") false false)
        ;[1 1 1] Detach From Sphere
        (if (Variables|Default|GetBreak)
          (Transformation|DetachFromComponent _destructible "KeepWorld" "KeepWorld" "KeepWorld" true)
          (else
            (Transformation|AttachComponentToComponent _destructible (Variables|Default|GetSphere) "None" "SnapToTarget" "SnapToTarget" "KeepWorld" true)))))))

(event EventBeginPlay
  ;[1 1 1] Start Custom Event
  (if (Variables|Default|GetActiveCart)
    (CallFunction|MoveCart)))

(fn ConstructionScript)