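; Animated mine cart actor that rides along a referenced track's spline.
; On BeginPlay, if the cart is active, a timeline starts from a configurable start offset with its play rate set from the Duration variable.
; Each update maps the timeline alpha to a distance along the spline and sets the cart's world location and rotation to match.
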(event Custom|MoveCart
  (bind _trackrefrence (Variables|Default|GetTrackRefrence))
  (bind _spline (Variables|/Game/Assets/ART_Blueprints/Paul_BP/BP_RoadBuilder.BP_RoadBuilder_C|GetSpline _trackrefrence))
  (Components|Timeline|SetPlayRate (Variables|Default|GetCartMover) (/ 1.0 (Variables|Default|GetDuration)))
  (Components|Timeline|SetNewTime (Variables|Default|GetCartMover) (Variables|Default|GetCartStartOffSet))
  (bind _alpha (Timeline|CartMover Play)
    (:Update
      (Variables|Default|SetAlpha _alpha)
      (Transformation|SetActorLocationAndRotation (Spline|GetLocationatDistanceAlongSpline _spline (Math|Float|Lerp 0.0 (Spline|GetSplineLength _spline) (Variables|Default|GetAlpha)) "World") (Spline|GetRotationatDistanceAlongSpline _spline (Math|Float|Lerp 0.0 (Spline|GetSplineLength _spline) (Variables|Default|GetAlpha)) "World")))))

(event EventBeginPlay
  (if (Variables|Default|GetActiveCart)
    (CallFunction|MoveCart)))

(fn ConstructionScript)