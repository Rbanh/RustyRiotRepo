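; Animated mine cart actor that travels along the MineSpline of a referenced track actor.
; When flagged active, it starts a timeline on BeginPlay, with play rate derived from Duration and start time set by an offset.
; Each timeline update maps alpha to distance along the spline, setting the cart's world location and rotation to match the track.
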(event Custom|MoveCart
  (bind _trackrefrence (Variables|Default|GetTrackRefrence))
  (bind _minespline (Variables|/Game/Assets/ART_Blueprints/MineCarts/BP_AnimTrack_JAB.BP_AnimTrack_JAB_C|GetMineSpline _trackrefrence))
  (Components|Timeline|SetPlayRate (Variables|Default|GetCartMover) (/ 1.0 (Variables|Default|GetDuration)))
  (Components|Timeline|SetNewTime (Variables|Default|GetCartMover) (Variables|Default|GetCartStartOffSet))
  (bind _alpha (Timeline|CartMover Play)
    (:Update
      (Variables|Default|SetAlpha _alpha)
      (Transformation|SetActorLocationAndRotation (Spline|GetLocationatDistanceAlongSpline _minespline (Math|Float|Lerp 0.0 (Spline|GetSplineLength _minespline) (Variables|Default|GetAlpha)) "World") (Spline|GetRotationatDistanceAlongSpline _minespline (Math|Float|Lerp 0.0 (Spline|GetSplineLength _minespline) (Variables|Default|GetAlpha)) "World")))))

(event EventBeginPlay
  (if (Variables|Default|GetActiveCart)
    (CallFunction|MoveCart)))

(fn ConstructionScript)