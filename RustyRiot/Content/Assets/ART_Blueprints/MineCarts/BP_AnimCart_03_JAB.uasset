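; Animated mine cart that rides along a referenced track's spline and breaks free when damaged.
; When active at BeginPlay, a timeline with duration-based play rate and start offset drives a sphere's position and rotation by spline distance.
; Each update snaps the destructible cart to the sphere until a hit or fracture sets a break flag, after which it detaches in world space.
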(event OnComponentFracture(Destructible)
  (params (HitPoint :type Vector%20%28by%20ref%29 :default "0, 0, 0") (HitDirection :type Vector%20%28by%20ref%29 :default "0, 0, 0"))
  (Variables|Default|SetBreak true))

(event OnComponentHit(Destructible)
  (params (HitComponent :type Primitive%20Component%20Object%20Reference) (OtherActor :type Actor%20Object%20Reference) (OtherComp :type Primitive%20Component%20Object%20Reference) (NormalImpulse :type Vector :default "0, 0, 0") (Hit :type Hit%20Result%20Structure%20%28by%20ref%29))
  (Variables|Default|SetBreak true))

(event Custom|MoveCart
  (bind _trackrefrence (Variables|Default|GetTrackRefrence))
  (bind _destructible (Variables|Default|GetDestructible))
  (bind _spline (Variables|/Game/Assets/ART_Blueprints/Paul_BP/BP_RoadBuilder.BP_RoadBuilder_C|GetSpline _trackrefrence))
  (Components|Timeline|SetPlayRate (Variables|Default|GetCartMover) (/ 1.0 (Variables|Default|GetDuration)))
  (Components|Timeline|SetNewTime (Variables|Default|GetCartMover) (Variables|Default|GetCartStartOffSet))
  (bind _alpha (Timeline|CartMover Play)
    (:Update
      (Variables|Default|SetAlpha _alpha)
      (Transformation|SetWorldLocationAndRotation (Variables|Default|GetSphere) (Spline|GetLocationatDistanceAlongSpline _spline (Math|Float|Lerp 0.0 (Spline|GetSplineLength _spline) (Variables|Default|GetAlpha)) "World") (Spline|GetRotationatDistanceAlongSpline _spline (Math|Float|Lerp 0.0 (Spline|GetSplineLength _spline) (Variables|Default|GetAlpha)) "World") false false)
      (if (Variables|Default|GetBreak)
        (Transformation|DetachFromComponent _destructible "KeepWorld" "KeepWorld" "KeepWorld" true)
        (else
          (Transformation|AttachComponentToComponent _destructible (Variables|Default|GetSphere) "None" "SnapToTarget" "SnapToTarget" "KeepWorld" true))))))

(event EventBeginPlay
  (if (Variables|Default|GetActiveCart)
    (CallFunction|MoveCart)))

(fn ConstructionScript)