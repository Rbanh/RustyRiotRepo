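; BP_LampCable_JAB is a configurable lamp on a cable, with a bulb mesh and a pulsing point light.
; The construction script sets up the meshes, bulb dynamic material, light and cable look from variables, and limits the physics constraint to the cable length.
; Each Tick, one time-based sine wave, offset by Floor, drives both light intensity and bulb color so they pulse in sync.
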(event EventTick
  (params (DeltaSeconds :type Float%20%28single-precision%29))
  (bind _returnvalue (Utilities|Time|GetGameTimeinSeconds))
  (bind _floor (Variables|Light|GetFloor))
  (bind _period (Variables|Light|GetPeriod))
  (bind _returnvalue_2 (* _returnvalue _period))
  (bind _returnvalue_3 (Math|Trig|Sin(Radians) _returnvalue_2))
  (bind _returnvalue_4 (+ _returnvalue_3 _floor))
  (Rendering|Components|Light|SetIntensity (Variables|Default|GetPointLight) (* _returnvalue_4 (Variables|Light|GetIntensity)))
  (Rendering|Material|SetVectorParameterValue (Variables|Default|GetDynamicMaterial) "Color" (* (Variables|Light|GetColor) _returnvalue_4) :!class /Script/Engine.MaterialInstanceDynamic))

(fn ConstructionScript
  (bind _physicsconstraint (Variables|Default|GetPhysicsConstraint))
  (bind _pointlight (Variables|Default|GetPointLight))
  (bind _bulp (Variables|Default|GetBulp))
  (bind _bulp_2 (Variables|Default|GetBulp))
  (bind _cable (Variables|Default|GetCable))
  (bind _cable_length (Variables|Cable|GetCable%20Length))
  (bind _bulp_material (Variables|Bulp|GetBulp%20Material))
  ;[1 1 1] Set Up the Lamp Mesh
  (Components|StaticMesh|SetStaticMesh (Variables|Default|GetLamp) (Variables|Lamp|GetLamp_Mesh))
  (Transformation|SetRelativeLocation (Variables|Default|GetLamp) (Math|Vector|MakeVector 0.0 0.0 (Variables|Lamp|GetLamp%20Location)) false false)
  (Transformation|SetRelativeScale3D (Variables|Default|GetLamp) (Math|Conversions|ToVector(Float) (Variables|Lamp|GetLamp%20Scale)))
  ;[1 1 1] Set Up Bulp Mesh
  (Components|StaticMesh|SetStaticMesh _bulp (Variables|Bulp|GetBulp%20mesh))
  (Transformation|SetRelativeLocation _bulp (Math|Vector|MakeVector 0.0 0.0 (Variables|Bulp|GetBulp%20Location)) false false)
  (Transformation|SetRelativeScale3D _bulp (Math|Conversions|ToVector(Float) (Variables|Bulp|GetBulp%20Scale)))
  (Class|PrimitiveComponent|SetCullDistance _bulp (Variables|Bulp|GetMesh%20Cull%20Distance))
  ;[1 1 1] Set Up Bulp material
  (Rendering|Material|SetMaterial _bulp_2 0 _bulp_material)
  (bind _returnvalue (Rendering|Material|CreateDynamicMaterialInstance _bulp_2 0 _bulp_material "None" :!class /Script/Engine.PrimitiveComponent))
  (bind _output_get (Variables|Default|SetDynamicMaterial _returnvalue))
  (Rendering|Material|SetVectorParameterValue _output_get "Color" (Variables|Light|GetColor) :!class /Script/Engine.MaterialInstanceDynamic)
  (Rendering|Material|SetScalarParameterValue _output_get "Distance" (Variables|Bulp|GetColor%20Cull%20Distance) :!class /Script/Engine.MaterialInstanceDynamic)
  ;[1 1 1] Set up Point Light
  (Transformation|AddRelativeLocation _pointlight (Math|Vector|MakeVector 0.0 0.0 (Variables|Light|GetLight%20Location)) false false)
  (Rendering|Components|Light|SetLightColor _pointlight (Variables|Light|GetColor) true)
  (Rendering|Components|Light|SetIntensity _pointlight (Variables|Light|GetIntensity))
  (Rendering|Lighting|SetAttenuationRadius _pointlight (Variables|Light|GetAttenuation%20Radius))
  (Rendering|Components|Light|SetLightFunctionMaterial _pointlight (Variables|Light|GetLight%20Function%20Material))
  ;[1 1 1] Set Up Cable Constrain Limits
  (Class|PhysicsConstraintComponent|SetLinearXLimit _physicsconstraint "LCM_Limited" _cable_length)
  (Class|PhysicsConstraintComponent|SetLinearYLimit _physicsconstraint "LCM_Limited" _cable_length)
  (Class|PhysicsConstraintComponent|SetLinearZLimit _physicsconstraint "LCM_Limited" _cable_length)
  ;[1 1 1] Set Up Cable
  (Rendering|Material|SetMaterial _cable 0 (Variables|Cable|GetCable%20Material))
  (Variables|/Script/CableComponent.CableComponent|SetTileMaterial _cable (Variables|Cable|GetTile%20Material%20Size))
  (Variables|/Script/CableComponent.CableComponent|SetCableWidth _cable (Variables|Cable|GetCable%20Width)))