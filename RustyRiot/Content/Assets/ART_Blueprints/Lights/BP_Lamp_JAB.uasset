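; BP_Lamp_JAB is a lamp actor with a point light and bulb mesh that pulse continuously over time.
; The construction script creates a dynamic bulb material and applies the configurable color, intensity, attenuation radius, light function and cull distances.
; Each tick, a sine of game time, scaled by Period and offset by Floor, modulates both the light intensity and the material's Color parameter, keeping glow and illumination in sync.
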(event EventTick
  (params (DeltaSeconds :type Float%20%28single-precision%29))
  (bind _returnvalue (Utilities|Time|GetGameTimeinSeconds))
  (bind _floor (Variables|Default|GetFloor))
  (bind _period (Variables|Default|GetPeriod))
  (bind _returnvalue_2 (* _returnvalue _period))
  (bind _returnvalue_3 (Math|Trig|Sin(Radians) _returnvalue_2))
  (bind _returnvalue_4 (+ _returnvalue_3 _floor))
  (Rendering|Components|Light|SetIntensity (Variables|Default|GetPointLight) (* _returnvalue_4 (Variables|Light|GetIntensity)))
  (Rendering|Material|SetVectorParameterValue (Variables|Default|GetDynamicMaterial) "Color" (* (Variables|Default|GetColor) _returnvalue_4) :!class /Script/Engine.MaterialInstanceDynamic))

(fn ConstructionScript
  (bind _returnvalue (Rendering|Material|CreateDynamicMaterialInstance (Variables|Default|GetBulp) 0 (Variables|Default|GetBulp%20Material) "None" :!class /Script/Engine.PrimitiveComponent))
  (bind _output_get (Variables|Default|SetDynamicMaterial _returnvalue))
  (Rendering|Material|SetVectorParameterValue _output_get "Color" (Variables|Default|GetColor) :!class /Script/Engine.MaterialInstanceDynamic)
  (Rendering|Material|SetScalarParameterValue _output_get "Distance" (Variables|Bulp|GetColor%20Cull%20Distance) :!class /Script/Engine.MaterialInstanceDynamic)
  (Rendering|Components|Light|SetLightColor (Variables|Default|GetPointLight) (Variables|Default|GetColor) true)
  (Rendering|Components|Light|SetIntensity (Variables|Default|GetPointLight) (Variables|Light|GetIntensity))
  (Rendering|Lighting|SetAttenuationRadius (Variables|Default|GetPointLight) (Variables|Light|GetAttenuation%20Radius))
  (Rendering|Components|Light|SetLightFunctionMaterial (Variables|Default|GetPointLight) (Variables|Default|GetLight%20Function%20Material))
  (Class|PrimitiveComponent|SetCullDistance (Variables|Default|GetBulp) (Variables|Bulp|GetMesh%20Cull%20Distance)))