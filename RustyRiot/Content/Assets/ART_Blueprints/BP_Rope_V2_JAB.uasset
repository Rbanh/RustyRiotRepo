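; BP_Rope_V2_JAB is a rope art Blueprint that builds itself by placing mesh instances along a spline.
; The construction script steps along the spline at Spacing intervals, adding a world-space Hierarchical Instanced Static Mesh instance aligned to the spline's rotation.
; Each instance gets a uniform scale between Min and Max from a random stream, so variation is repeatable.
; The event graph has no runtime logic.
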(event EventBeginPlay)

(event Collision|EventActorBeginOverlap
  (params (OtherActor :type Actor%20Object%20Reference)))

(event EventTick
  (params (DeltaSeconds :type Float%20%28single-precision%29)))

(fn ConstructionScript
  (bind _spline (Variables|Default|GetSpline))
  (bind _spacing (Variables|Mesh|Getspacing))
  (for _index (range 1 (.ReturnValue (Math|Float|Division(WholeandRemainder) (Spline|GetSplineLength _spline) _spacing)))
    (Class|InstancedStaticMeshComponent|AddInstanceWorldSpace (Variables|Default|GetHierarchicalInstancedStaticMesh) (Math|Transform|MakeTransform (Spline|GetLocationatDistanceAlongSpline _spline (* (Math|Conversions|ToFloat(Integer) _index) _spacing) "World") (Spline|GetRotationatDistanceAlongSpline _spline (* (Math|Conversions|ToFloat(Integer) _index) _spacing) "World") (Math|Conversions|ToVector(Float) (Math|Random|RandomFloatinRangefromStream (Variables|Mesh|GetMin) (Variables|Mesh|GetMax) (Variables|Default|GetRandomStream)))))))