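; Spline-based power line builder that places a BP_PowerLine_JAB child actor at every spline point, oriented along the spline, in the construction script.
; A first loop applies the shared mesh, materials, connector offsets and cable settings to each pole.
; A second loop strings two cables between neighboring poles' connectors, sizing each to their distance plus random slack, and zeroes the last pole's cables.
; The Scale assignment is unconnected.
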(event EventBeginPlay)

(event Collision|EventActorBeginOverlap
  (params (OtherActor :type Actor%20Object%20Reference)))

(event EventTick
  (params (DeltaSeconds :type Float%20%28single-precision%29)))

(fn ConstructionScript
  (bind _spline (Variables|Default|GetSpline))
  (bind _tile_material (Variables|Cable|GetTile%20Material))
  (bind _enable_stiffness (Variables|Cable|GetEnable%20Stiffness))
  (bind _enable_collision (Variables|Cable|GetEnable%20Collision))
  (bind _cable_width (Variables|Cable|GetCable%20Width))
  (bind _location_2 (Variables|Cable|GetLocation%202))
  (bind _location_1 (Variables|Cable|GetLocation%201))
  (bind _solver_iterations (Variables|Cable|GetSolver%20Iterations))
  (bind _output_get (Variables|Default|SetNumber%20of%20Spline%20Points (- (Spline|GetNumberOfSplinePoints (Variables|Default|GetSpline)) 1)))
  (for _index (range 0 _output_get)
    (Variables|Default|SetIndex%20of%20Loop _index)
    (bind _returnvalue (AddComponent|AddChildActorComponent false (Math|Conversions|ToTransform(Vector) (Spline|GetLocationatSplinePoint _spline (Variables|Default|GetIndex%20of%20Loop) "Local"))))
    (ChildActorComponent|SetChildActorClass _returnvalue "/Game/Assets/ART_Blueprints/PowerLine/BP_PowerLine_JAB.BP_PowerLine_JAB_C")
    (bind _asbp_power_line_jab (Utilities|Casting|CastToBP_PowerLine_JAB (Variables|/Script/Engine.ChildActorComponent|GetChildActor _returnvalue)))
    (Components|StaticMesh|SetStaticMesh (Variables|/Game/Assets/ART_Blueprints/PowerLine/BP_PowerLine_JAB.BP_PowerLine_JAB_C|GetStaticMesh _asbp_power_line_jab) (Variables|Mesh|GetMesh%20Object))
    (Rendering|Material|SetMaterial (Variables|/Game/Assets/ART_Blueprints/PowerLine/BP_PowerLine_JAB.BP_PowerLine_JAB_C|GetStaticMesh _asbp_power_line_jab) 0 (Variables|Mesh|GetMesh%20Material))
    (Utilities|Array|Add (Variables|Default|GetAll%20Child%20Actors%20of%20powerLine) _asbp_power_line_jab)
    (Transformation|SetRelativeRotation _returnvalue (Spline|GetRotationatSplinePoint _spline (Variables|Default|GetIndex%20of%20Loop) "Local") false false)
    (Utilities|FlowControl|Sequence
      (:then_0
        (Transformation|SetRelativeLocation (Variables|/Game/Assets/ART_Blueprints/PowerLine/BP_PowerLine_JAB.BP_PowerLine_JAB_C|GetCon1 (Utilities|Array|Get(acopy) (Variables|Default|GetAll%20Child%20Actors%20of%20powerLine) (Variables|Default|GetIndex%20of%20Loop))) _location_1 false false))
      (:then_1
        (Variables|/Script/CableComponent.CableComponent|SetEndLocation (Variables|/Game/Assets/ART_Blueprints/PowerLine/BP_PowerLine_JAB.BP_PowerLine_JAB_C|GetCable1 (Utilities|Array|Get(acopy) (Variables|Default|GetAll%20Child%20Actors%20of%20powerLine) (Variables|Default|GetIndex%20of%20Loop))) _location_1))
      (:then_2
        (Transformation|SetRelativeLocation (Variables|/Game/Assets/ART_Blueprints/PowerLine/BP_PowerLine_JAB.BP_PowerLine_JAB_C|GetCon2 (Utilities|Array|Get(acopy) (Variables|Default|GetAll%20Child%20Actors%20of%20powerLine) (Variables|Default|GetIndex%20of%20Loop))) _location_2 false false))
      (:then_3
        (Variables|/Script/CableComponent.CableComponent|SetEndLocation (Variables|/Game/Assets/ART_Blueprints/PowerLine/BP_PowerLine_JAB.BP_PowerLine_JAB_C|GetCable2 (Utilities|Array|Get(acopy) (Variables|Default|GetAll%20Child%20Actors%20of%20powerLine) (Variables|Default|GetIndex%20of%20Loop))) _location_2))
      (:then_4
        (Rendering|Material|SetMaterial (Variables|/Game/Assets/ART_Blueprints/PowerLine/BP_PowerLine_JAB.BP_PowerLine_JAB_C|GetCable1 (Utilities|Array|Get(acopy) (Variables|Default|GetAll%20Child%20Actors%20of%20powerLine) (Variables|Default|GetIndex%20of%20Loop))) 0 (Variables|Cable|GetCable%20Material))
        (Utilities|FlowControl|Sequence
          (:then_0
            (Variables|/Script/CableComponent.CableComponent|SetTileMaterial (Variables|/Game/Assets/ART_Blueprints/PowerLine/BP_PowerLine_JAB.BP_PowerLine_JAB_C|GetCable1 (Utilities|Array|Get(acopy) (Variables|Default|GetAll%20Child%20Actors%20of%20powerLine) (Variables|Default|GetIndex%20of%20Loop))) _tile_material)
            (Variables|/Script/CableComponent.CableComponent|SetCableWidth (Variables|/Game/Assets/ART_Blueprints/PowerLine/BP_PowerLine_JAB.BP_PowerLine_JAB_C|GetCable1 (Utilities|Array|Get(acopy) (Variables|Default|GetAll%20Child%20Actors%20of%20powerLine) (Variables|Default|GetIndex%20of%20Loop))) _cable_width)
            (Variables|/Script/CableComponent.CableComponent|SetbEnableStiffness (Variables|/Game/Assets/ART_Blueprints/PowerLine/BP_PowerLine_JAB.BP_PowerLine_JAB_C|GetCable1 (Utilities|Array|Get(acopy) (Variables|Default|GetAll%20Child%20Actors%20of%20powerLine) (Variables|Default|GetIndex%20of%20Loop))) _enable_stiffness)
            (Variables|/Script/CableComponent.CableComponent|SetbEnableCollision (Variables|/Game/Assets/ART_Blueprints/PowerLine/BP_PowerLine_JAB.BP_PowerLine_JAB_C|GetCable1 (Utilities|Array|Get(acopy) (Variables|Default|GetAll%20Child%20Actors%20of%20powerLine) (Variables|Default|GetIndex%20of%20Loop))) _enable_collision)
            (Variables|/Script/CableComponent.CableComponent|SetSolverIterations (Variables|/Game/Assets/ART_Blueprints/PowerLine/BP_PowerLine_JAB.BP_PowerLine_JAB_C|GetCable1 (Utilities|Array|Get(acopy) (Variables|Default|GetAll%20Child%20Actors%20of%20powerLine) (Variables|Default|GetIndex%20of%20Loop))) _solver_iterations))
          (:then_1
            (Variables|/Script/CableComponent.CableComponent|SetTileMaterial (Variables|/Game/Assets/ART_Blueprints/PowerLine/BP_PowerLine_JAB.BP_PowerLine_JAB_C|GetCable2 (Utilities|Array|Get(acopy) (Variables|Default|GetAll%20Child%20Actors%20of%20powerLine) (Variables|Default|GetIndex%20of%20Loop))) _tile_material)
            (Variables|/Script/CableComponent.CableComponent|SetCableWidth (Variables|/Game/Assets/ART_Blueprints/PowerLine/BP_PowerLine_JAB.BP_PowerLine_JAB_C|GetCable2 (Utilities|Array|Get(acopy) (Variables|Default|GetAll%20Child%20Actors%20of%20powerLine) (Variables|Default|GetIndex%20of%20Loop))) _cable_width)
            (Variables|/Script/CableComponent.CableComponent|SetbEnableStiffness (Variables|/Game/Assets/ART_Blueprints/PowerLine/BP_PowerLine_JAB.BP_PowerLine_JAB_C|GetCable2 (Utilities|Array|Get(acopy) (Variables|Default|GetAll%20Child%20Actors%20of%20powerLine) (Variables|Default|GetIndex%20of%20Loop))) _enable_stiffness)
            (Variables|/Script/CableComponent.CableComponent|SetbEnableCollision (Variables|/Game/Assets/ART_Blueprints/PowerLine/BP_PowerLine_JAB.BP_PowerLine_JAB_C|GetCable2 (Utilities|Array|Get(acopy) (Variables|Default|GetAll%20Child%20Actors%20of%20powerLine) (Variables|Default|GetIndex%20of%20Loop))) _enable_collision)
            (Variables|/Script/CableComponent.CableComponent|SetSolverIterations (Variables|/Game/Assets/ART_Blueprints/PowerLine/BP_PowerLine_JAB.BP_PowerLine_JAB_C|GetCable2 (Utilities|Array|Get(acopy) (Variables|Default|GetAll%20Child%20Actors%20of%20powerLine) (Variables|Default|GetIndex%20of%20Loop))) _solver_iterations))))))
  (for _index_2 (range 0 (Variables|Default|GetNumber%20of%20Spline%20Points))
    (Variables|Default|SetIndex%20Loop%202 _index_2)
    (Utilities|FlowControl|Sequence
      (:then_0
        (Transformation|AttachComponentToComponent (Variables|/Game/Assets/ART_Blueprints/PowerLine/BP_PowerLine_JAB.BP_PowerLine_JAB_C|GetCable1 (Utilities|Array|Get(acopy) (Variables|Default|GetAll%20Child%20Actors%20of%20powerLine) (Variables|Default|GetIndex%20Loop%202))) (Variables|/Game/Assets/ART_Blueprints/PowerLine/BP_PowerLine_JAB.BP_PowerLine_JAB_C|GetCon1 (Utilities|Array|Get(acopy) (Variables|Default|GetAll%20Child%20Actors%20of%20powerLine) (+ (Variables|Default|GetIndex%20Loop%202) 1))) "None" "SnapToTarget" "SnapToTarget" "KeepWorld" true)
        (Variables|/Script/CableComponent.CableComponent|SetCableLength (Variables|/Game/Assets/ART_Blueprints/PowerLine/BP_PowerLine_JAB.BP_PowerLine_JAB_C|GetCable1 (Utilities|Array|Get(acopy) (Variables|Default|GetAll%20Child%20Actors%20of%20powerLine) (Variables|Default|GetIndex%20Loop%202))) (+ (Math|Random|RandomFloatinRange 0.0 (Variables|Cable|GetRandom%20Slack%201)) (Math|Vector|VectorLength (- (Transformation|GetWorldLocation (Variables|/Game/Assets/ART_Blueprints/PowerLine/BP_PowerLine_JAB.BP_PowerLine_JAB_C|GetCon1 (Utilities|Array|Get(acopy) (Variables|Default|GetAll%20Child%20Actors%20of%20powerLine) (Variables|Default|GetIndex%20Loop%202)))) (Transformation|GetWorldLocation (Variables|/Game/Assets/ART_Blueprints/PowerLine/BP_PowerLine_JAB.BP_PowerLine_JAB_C|GetCon1 (Utilities|Array|Get(acopy) (Variables|Default|GetAll%20Child%20Actors%20of%20powerLine) (+ (Variables|Default|GetIndex%20Loop%202) 1))))))))
        (Variables|/Script/CableComponent.CableComponent|SetCableLength (Variables|/Game/Assets/ART_Blueprints/PowerLine/BP_PowerLine_JAB.BP_PowerLine_JAB_C|GetCable1 (Utilities|Array|Get(acopy) (Variables|Default|GetAll%20Child%20Actors%20of%20powerLine) (Variables|Default|GetNumber%20of%20Spline%20Points))) 0.0)
        (Transformation|SetRelativeLocation (Variables|/Game/Assets/ART_Blueprints/PowerLine/BP_PowerLine_JAB.BP_PowerLine_JAB_C|GetCable1 (Utilities|Array|Get(acopy) (Variables|Default|GetAll%20Child%20Actors%20of%20powerLine) (Variables|Default|GetNumber%20of%20Spline%20Points))) (Variables|Cable|GetLocation%201) false false)
        (Variables|/Script/CableComponent.CableComponent|SetbEnableCollision (Variables|/Game/Assets/ART_Blueprints/PowerLine/BP_PowerLine_JAB.BP_PowerLine_JAB_C|GetCable1 (Utilities|Array|Get(acopy) (Variables|Default|GetAll%20Child%20Actors%20of%20powerLine) (Variables|Default|GetNumber%20of%20Spline%20Points))) false))
      (:then_1
        (Transformation|AttachComponentToComponent (Variables|/Game/Assets/ART_Blueprints/PowerLine/BP_PowerLine_JAB.BP_PowerLine_JAB_C|GetCable2 (Utilities|Array|Get(acopy) (Variables|Default|GetAll%20Child%20Actors%20of%20powerLine) (Variables|Default|GetIndex%20Loop%202))) (Variables|/Game/Assets/ART_Blueprints/PowerLine/BP_PowerLine_JAB.BP_PowerLine_JAB_C|GetCon2 (Utilities|Array|Get(acopy) (Variables|Default|GetAll%20Child%20Actors%20of%20powerLine) (+ (Variables|Default|GetIndex%20Loop%202) 1))) "None" "SnapToTarget" "SnapToTarget" "KeepWorld" true)
        (Variables|/Script/CableComponent.CableComponent|SetCableLength (Variables|/Game/Assets/ART_Blueprints/PowerLine/BP_PowerLine_JAB.BP_PowerLine_JAB_C|GetCable2 (Utilities|Array|Get(acopy) (Variables|Default|GetAll%20Child%20Actors%20of%20powerLine) (Variables|Default|GetIndex%20Loop%202))) (+ (Math|Random|RandomFloatinRange 0.0 (Variables|Cable|GetRandom%20Slack%202)) (Math|Vector|VectorLength (- (Transformation|GetWorldLocation (Variables|/Game/Assets/ART_Blueprints/PowerLine/BP_PowerLine_JAB.BP_PowerLine_JAB_C|GetCon2 (Utilities|Array|Get(acopy) (Variables|Default|GetAll%20Child%20Actors%20of%20powerLine) (Variables|Default|GetIndex%20Loop%202)))) (Transformation|GetWorldLocation (Variables|/Game/Assets/ART_Blueprints/PowerLine/BP_PowerLine_JAB.BP_PowerLine_JAB_C|GetCon2 (Utilities|Array|Get(acopy) (Variables|Default|GetAll%20Child%20Actors%20of%20powerLine) (+ (Variables|Default|GetIndex%20Loop%202) 1))))))))
        (Variables|/Script/CableComponent.CableComponent|SetCableLength (Variables|/Game/Assets/ART_Blueprints/PowerLine/BP_PowerLine_JAB.BP_PowerLine_JAB_C|GetCable2 (Utilities|Array|Get(acopy) (Variables|Default|GetAll%20Child%20Actors%20of%20powerLine) (Variables|Default|GetNumber%20of%20Spline%20Points))) 0.0)
        (Transformation|SetRelativeLocation (Variables|/Game/Assets/ART_Blueprints/PowerLine/BP_PowerLine_JAB.BP_PowerLine_JAB_C|GetCable2 (Utilities|Array|Get(acopy) (Variables|Default|GetAll%20Child%20Actors%20of%20powerLine) (Variables|Default|GetNumber%20of%20Spline%20Points))) (Variables|Cable|GetLocation%202) false false)
        (Variables|/Script/CableComponent.CableComponent|SetbEnableCollision (Variables|/Game/Assets/ART_Blueprints/PowerLine/BP_PowerLine_JAB.BP_PowerLine_JAB_C|GetCable2 (Utilities|Array|Get(acopy) (Variables|Default|GetAll%20Child%20Actors%20of%20powerLine) (Variables|Default|GetNumber%20of%20Spline%20Points))) false)))))