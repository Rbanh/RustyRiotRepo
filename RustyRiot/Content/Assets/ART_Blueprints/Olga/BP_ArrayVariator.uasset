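; BP_ArrayVariator is a scatter tool that fills a 3D grid with randomized instances of up to four meshes in its Construction Script.
; A seeded stream picks each cell's mesh or gap (via Skip) and varies offset, rotation and scale.
; Cell spacing follows Mesh1's bounds, and each mesh has its own HISM component.
; Placement_Macro adds instances, optionally snapping them to traced surfaces and tilting to the hit normal.
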(event EventBeginPlay)

(event Collision|EventActorBeginOverlap
  (params (OtherActor :type Actor%20Object%20Reference)))

(fn ConstructionScript
  (bind _randomshift (Variables|Default|GetRandomShift))
  (bind _randseed (LocalVariables|Getrandseed))
  (bind _randseed_2 (LocalVariables|Getrandseed))
  (bind _randseed_3 (LocalVariables|Getrandseed))
  (bind _hierarchicalinstancedstaticmesh (Variables|Default|GetHierarchicalInstancedStaticMesh))
  (bind _scale_all_each_rand (Variables|Default|GetScale:All/Each/Rand))
  (bind _mesh1 (Variables|Default|GetMesh1))
  (bind _scale_all_each_rand_2 (Variables|Default|GetScale:All/Each/Rand))
  (bind _hierarchicalinstancedstaticmesh1 (Variables|Default|GetHierarchicalInstancedStaticMesh1))
  (bind _hierarchicalinstancedstaticmesh2 (Variables|Default|GetHierarchicalInstancedStaticMesh2))
  (bind _shift (Variables|Default|GetShift))
  (bind _hierarchicalinstancedstaticmesh3 (Variables|Default|GetHierarchicalInstancedStaticMesh3))
  (bind _randomrotate (Variables|Default|GetRandomRotate))
  (bind _returnvalue (Math|Random|RandomFloatfromStream _randseed_2))
  (bind _returnvalue_2 (Math|Random|RandomFloatinRangefromStream -1.8e+02 1.8e+02 _randseed_3))
  (bind _returnvalue_3 (Math|Random|RandomUnitVectorfromStream _randseed))
  (bind _returnvalue_4 (StaticMesh|GetBoundingBox _mesh1))
  (bind _returnvalue_5 (* (.x _scale_all_each_rand_2) (.y _scale_all_each_rand_2)))
  (bind (_min _max) (Utilities|Struct|BreakBox _returnvalue_4))
  (bind _returnvalue_6 (- _returnvalue_5 (.z _scale_all_each_rand_2)))
  (bind _returnvalue_7 (* _returnvalue_2 0.01))
  (bind _returnvalue_8 (* (Math|Vector|MakeVector (.x _randomshift) (.x _randomshift) (.y _randomshift)) _returnvalue_3))
  (bind _returnvalue_9 (* (.z _scale_all_each_rand_2) _returnvalue))
  (bind _returnvalue_10 (* (Math|Rotator|MakeRotator (.y _randomrotate) (.y _randomrotate) (.x _randomrotate)) _returnvalue_7))
  (bind _returnvalue_11 (- _max _min))
  (bind _returnvalue_12 (+ _returnvalue_6 _returnvalue_9))
  (bind _returnvalue_13 (Math|Float|Absolute(Float) _returnvalue_12))
  (bind _returnvalue_14 (+ _returnvalue_11 _shift))
  (bind _returnvalue_15 (* _returnvalue_14 (.x _scale_all_each_rand)))
  (bind _returnvalue_16 (Math|Vector|MakeVector _returnvalue_13 _returnvalue_13 _returnvalue_13))
  ;[1 1 1] set random seed
  (Math|Random|SetRandomStreamSeed (LocalVariables|Getrandseed) (Variables|Default|GetSeed))
  ;[1 1 1] set volume
  (for _index (range 0 (Utilities|FixCount (Variables|Default|GetWidth)))
    (for _index_2 (range 0 (Utilities|FixCount (Variables|Default|GetLength)))
      (for _index_3 (range 0 (Utilities|FixCount (Variables|Default|GetHeight)))
        ;[1 1 1] getting known how many meshes plugged
        (if (!= (Variables|Default|GetMesh4) 0)
          (LocalVariables|Setmeshes%20count 3)
          (elif (!= (Variables|Default|GetMesh3) 0)
            (LocalVariables|Setmeshes%20count 2)
            (elif (!= (Variables|Default|GetMesh2) 0)
              (LocalVariables|Setmeshes%20count 1)
              (else
                (LocalVariables|Setmeshes%20count 0)))))
        ;[1 1 1] skip
        (LocalVariables|Setmeshes%20count (+ (LocalVariables|Getmeshes%20count) (+ (Variables|Default|GetSkip) 1)))
        ;[1 1 1] random choosing mesh from list
        (switch int (Class|KismetMathLibrary|RandomIntegerfromStream (LocalVariables|Getmeshes%20count) (LocalVariables|Getrandseed))
          (:0
            (Components|StaticMesh|SetStaticMesh _hierarchicalinstancedstaticmesh (Variables|Default|GetMesh1))
            (Utilities|PlacementMacro _hierarchicalinstancedstaticmesh (+ (Math|Vector|MakeVector (* _index (.x _returnvalue_15)) (* _index_2 (.y _returnvalue_15)) (* _index_3 (.z _returnvalue_15))) (Math|Vector|MakeVector (.x _returnvalue_8) (.y _returnvalue_8) (.z _returnvalue_8))) _returnvalue_10 (Variables|Default|GetRotate1) _returnvalue_16))
          (:1
            (Components|StaticMesh|SetStaticMesh _hierarchicalinstancedstaticmesh1 (Variables|Default|GetMesh2))
            (Utilities|PlacementMacro _hierarchicalinstancedstaticmesh1 (+ (Math|Vector|MakeVector (* _index (.x _returnvalue_15)) (* _index_2 (.y _returnvalue_15)) (* _index_3 (.z _returnvalue_15))) (Math|Vector|MakeVector (.x _returnvalue_8) (.y _returnvalue_8) (.z _returnvalue_8))) _returnvalue_10 (Variables|Default|GetRotate2) _returnvalue_16))
          (:2
            (Components|StaticMesh|SetStaticMesh _hierarchicalinstancedstaticmesh2 (Variables|Default|GetMesh3))
            (Utilities|PlacementMacro _hierarchicalinstancedstaticmesh2 (+ (Math|Vector|MakeVector (* _index (.x _returnvalue_15)) (* _index_2 (.y _returnvalue_15)) (* _index_3 (.z _returnvalue_15))) (Math|Vector|MakeVector (.x _returnvalue_8) (.y _returnvalue_8) (.z _returnvalue_8))) _returnvalue_10 (Variables|Default|GetRotate3) _returnvalue_16))
          (:3
            (Components|StaticMesh|SetStaticMesh _hierarchicalinstancedstaticmesh3 (Variables|Default|GetMesh4))
            (Utilities|PlacementMacro _hierarchicalinstancedstaticmesh3 (+ (Math|Vector|MakeVector (* _index (.x _returnvalue_15)) (* _index_2 (.y _returnvalue_15)) (* _index_3 (.z _returnvalue_15))) (Math|Vector|MakeVector (.x _returnvalue_8) (.y _returnvalue_8) (.z _returnvalue_8))) _returnvalue_10 (Variables|Default|GetRotate4) _returnvalue_16)))))))