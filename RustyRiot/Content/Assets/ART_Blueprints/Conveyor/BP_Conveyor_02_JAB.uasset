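; Conveyor belt actor that pushes every actor overlapping its Box along the mesh's forward vector at Speed.
; Tick applies a frame-rate-scaled world offset, teleporting without sweep.
; Box begin and end overlaps both call SpeedBoost on actors matching any of three cast targets.
; The construction script builds a dynamic material instance for arrow color, scale and scroll speed, and sets the mesh's cull distance.
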(event OnComponentEndOverlap(Box)
  (params (OverlappedComponent :type Primitive%20Component%20Object%20Reference) (OtherActor :type Actor%20Object%20Reference) (OtherComp :type Primitive%20Component%20Object%20Reference) (OtherBodyIndex :type Integer))
  (Utilities|FlowControl|Sequence
    (:then_0
      (bind _assedan (Utilities|Casting|CastTo OtherActor))
      (CallFunction|SpeedBoost _assedan))
    (:then_1
      (bind _asmini_beast (Utilities|Casting|CastTo OtherActor))
      (CallFunction|SpeedBoost _asmini_beast))
    (:then_2
      (bind _asmini_beast_02 (Utilities|Casting|CastTo OtherActor))
      (CallFunction|SpeedBoost _asmini_beast_02))))

(event OnComponentBeginOverlap(Box)
  (params (OverlappedComponent :type Primitive%20Component%20Object%20Reference) (OtherActor :type Actor%20Object%20Reference) (OtherComp :type Primitive%20Component%20Object%20Reference) (OtherBodyIndex :type Integer) (bFromSweep :type Boolean) (SweepResult :type Hit%20Result%20Structure%20%28by%20ref%29))
  (Utilities|FlowControl|Sequence
    (:then_0
      (bind _assedan (Utilities|Casting|CastTo OtherActor))
      (CallFunction|SpeedBoost _assedan))
    (:then_1
      (bind _asmini_beast (Utilities|Casting|CastTo OtherActor))
      (CallFunction|SpeedBoost _asmini_beast))
    (:then_2
      (bind _asmini_beast_02 (Utilities|Casting|CastTo OtherActor))
      (CallFunction|SpeedBoost _asmini_beast_02))))

(event EventTick
  (params (DeltaSeconds :type Float%20%28single-precision%29))
  (for _array_element (Collision|GetOverlappingActors (Variables|Default|GetBox) 0 :!class /Script/Engine.PrimitiveComponent)
    (Transformation|AddActorWorldOffset _array_element (* (Math|Vector|GetForwardVector (Transformation|GetWorldRotation (Variables|Default|GetStaticMesh))) (* DeltaSeconds (Variables|Default|GetSpeed))) false true)))

(fn ConstructionScript
  (bind _staticmesh (Variables|Default|GetStaticMesh))
  (bind _returnvalue (Rendering|Material|CreateDynamicMaterialInstance _staticmesh 0 "/Game/Assets/MaterialInstances/MI_Conveyor_JAB.MI_Conveyor_JAB" "None" :!class /Script/Engine.PrimitiveComponent))
  (Rendering|Material|SetMaterial _staticmesh 0 _returnvalue)
  (Rendering|Material|SetVectorParameterValue _returnvalue "Color" (Variables|Default|GetColor) :!class /Script/Engine.MaterialInstanceDynamic)
  (Rendering|Material|SetScalarParameterValue _returnvalue "X Scale" (Variables|Default|GetArrows%20Scale) :!class /Script/Engine.MaterialInstanceDynamic)
  (Rendering|Material|SetScalarParameterValue _returnvalue "X Speed" (Variables|Default|GetArrows%20Speed) :!class /Script/Engine.MaterialInstanceDynamic)
  (Class|PrimitiveComponent|SetCullDistance (Variables|Default|GetStaticMesh) (Variables|Default|GetDraw%20Distance)))