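; Procedural house Blueprint that assembles a modular building in its construction script, with no active runtime logic.
; It adds a foundation, stacks wall meshes by the Floors count, caps them with a roof, and picks a door through DoorMacro from DoorStyle.
; Five 1stWin toggles add Window mesh instances at fixed spots, reused for upper-floor windows behind FloorCheckMacro, where toggle A excludes the others.
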(event EventBeginPlay)

(event Collision|EventActorBeginOverlap
  (params (OtherActor :type Actor%20Object%20Reference)))

(event EventTick
  (params (DeltaSeconds :type Float%20%28single-precision%29)))

(fn ConstructionScript
  (Utilities|FlowControl|Sequence
    (:then_0
      ;[1 1 1] Foundation
      (AddComponent|AddStaticMeshComponent false (Math|Transform|MakeTransform "-150.000000,-250.000000,-90.000000" "0.000000,90.000000,0.000000" "1,1,1"))
      ;[1 1 1] Walls
      (for _index (range 0 (Variables|Default|GetFloors))
        (AddComponent|AddStaticMeshComponent false (Math|Transform|MakeTransform (Math|Vector|MakeVector 2e+01 6e+01 (* _index 2.4e+02)) "0,90.000000, 0" "1,1,1")))
      ;[1 1 1] Roof Generation
      (AddComponent|AddStaticMeshComponent false (Math|Transform|MakeTransform (Math|Vector|MakeVector 2e+01 6e+01 (* _index 2.4e+02)) "0,90.000000, 0" "1,1,1")))
    (:then_1
      (Utilities|DoorMacro))
    (:then_2
      (Utilities|FloorCheckMacro
        (:Out
          (if (Variables|Default|Get1stWinA)
            (Components|InstancedStaticMesh|AddInstance (Variables|Default|GetWindow) (Math|Transform|MakeTransform "-155.000000,50.000000,300.000000" "0.000000,90.000000,0.000000" "1,1,1"))
            (else
              (if (Variables|Default|Get1stWinB)
                (Components|InstancedStaticMesh|AddInstance (Variables|Default|GetWindow) (Math|Transform|MakeTransform "-60.000000,215.000000,300.000000" "0.000000,180.000000,0.000000" "1,1,1")))
              (if (Variables|Default|Get1stWinC)
                (Components|InstancedStaticMesh|AddInstance (Variables|Default|GetWindow) (Math|Transform|MakeTransform "95.000000,215.000000,300.000000" "0.000000,-180.000000,0.000000" "1,1,1")))
              (if (Variables|Default|Get1stWinD)
                (Components|InstancedStaticMesh|AddInstance (Variables|Default|GetWindow) (Math|Transform|MakeTransform "200.000000,50.000000,300.000000" "0.000000,90.000000,0.000000" "1,1,1")))
              (if (Variables|Default|Get1stWinE)
                (Components|InstancedStaticMesh|AddInstance (Variables|Default|GetWindow) (Math|Transform|MakeTransform "60.000000,80.000000,300.000000" "0.000000,90.000000,0.000000" "1,1,1"))))))))
    (:then_3
      (if (Variables|Default|Get1stWinA)
        (Components|InstancedStaticMesh|AddInstance (Variables|Default|GetWindow) (Math|Transform|MakeTransform "-155.000000,50.000000,20.000000" "0.000000,90.000000,0.000000" "1,1,1")))
      (if (Variables|Default|Get1stWinB)
        (Components|InstancedStaticMesh|AddInstance (Variables|Default|GetWindow) (Math|Transform|MakeTransform "-60.000000,215.000000,20.000000" "0.000000,180.000000,0.000000" "1,1,1")))
      (if (Variables|Default|Get1stWinC)
        (Components|InstancedStaticMesh|AddInstance (Variables|Default|GetWindow) (Math|Transform|MakeTransform "95.000000,215.000000,20.000000" "0.000000,-180.000000,0.000000" "1,1,1")))
      (if (Variables|Default|Get1stWinD)
        (Components|InstancedStaticMesh|AddInstance (Variables|Default|GetWindow) (Math|Transform|MakeTransform "200.000000,50.000000,20.000000" "0.000000,90.000000,0.000000" "1,1,1")))
      (if (Variables|Default|Get1stWinE)
        (Components|InstancedStaticMesh|AddInstance (Variables|Default|GetWindow) (Math|Transform|MakeTransform "60.000000,80.000000,280.000000" "0.000000,90.000000,0.000000" "1,1,1"))))))