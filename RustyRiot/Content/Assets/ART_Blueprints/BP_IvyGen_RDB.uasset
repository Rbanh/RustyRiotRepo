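; Procedural ivy generator that builds a tapering branch with random leaves in the construction script, following an editable control spline.
; Each control point line-traces against WorldStatic along an arrow pitched 90 degrees down, forming a new spline from hit locations, with normals added to tangents.
; Spline meshes are laid at fixed spacing along that projected spline, with instanced leaves scattered by probability.
; Debug trace drawing and prints remain active.
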(event Custom|Collisioin%20HIt
  (params (Hit%20Actor :type Actor%20Object%20Reference))
  (Development|PrintString "Hello"))

(event EventBeginPlay)

(event Collision|EventActorBeginOverlap
  (params (OtherActor :type Actor%20Object%20Reference)))

(event EventTick
  (params (DeltaSeconds :type Float%20%28single-precision%29)))

(fn ConstructionScript
  (bind _spacing (Variables|Default|GetSpacing))
  (bind _spacing_2 (Variables|Default|GetSpacing))
  (bind _branchthickness (Variables|Default|GetBranchThickness))
  (CallFunction|GetSplinePoints)
  (bind _returnvalue (AddComponent|AddSplineComponent false))
  (bind _output_get (Variables|Default|SetMainSpline _returnvalue))
  (Spline|ClearSplinePoints _output_get true)
  (for (_array_element _array_index) (Variables|Default|GetSplinePoints)
    (bind _returnvalue_2 (AddComponent|AddArrowComponent false (Math|Transform|MakeTransform (.position _array_element) (Math|Rotator|MakeRotator (.roll (.rotation _array_element)) (+ (.pitch (.rotation _array_element)) -9e+01) (.yaw (.rotation _array_element))) "1,1,1")))
    (Variables|Default|SettraceDirection (Math|Vector|GetForwardVector _returnvalue_2))
    (bind (_outhit _returnvalue_3) (Collision|LineTraceForObjects (Transformation|GetWorldLocation _returnvalue_2) (+ (Transformation|GetWorldLocation _returnvalue_2) (* (Math|Vector|GetForwardVector _returnvalue_2) (Variables|Default|GetTraceRange))) (Utilities|Array|MakeArray "ObjectTypeQuery1") false 0 "ForDuration" true "(R=0.020887,G=0.000000,B=1.000000,A=1.000000)" "(R=0.000000,G=0.065865,B=1.000000,A=1.000000)" 1.0))
    (Development|PrintString (Utilities|GetDisplayName (.hitactor _outhit)))
    (Spline|AddSplinePointatIndex (Variables|Default|GetMainSpline) (Math|Vector|SelectVector (.location _outhit) (- (Transformation|GetWorldLocation _returnvalue_2) "0, 0,10.000000") _returnvalue_3) _array_index "World" true)
    (Spline|SetTangentsatSplinePoint (Variables|Default|GetMainSpline) _array_index (+ (.normal _outhit) (.arrivetangent (Utilities|Array|Get(acopy) (Variables|Default|GetSplinePoints) _array_index))) (+ (.normal _outhit) (.leavetangent (Utilities|Array|Get(acopy) (Variables|Default|GetSplinePoints) _array_index))) "World" true))
  (Variables|Default|SetLeaf (Variables|Default|GetLeafMesh))
  (for _index (range 0 (.ReturnValue (Math|Float|Division(WholeandRemainder) (Spline|GetSplineLength (Variables|Default|GetMainSpline)) _spacing_2)))
    (Variables|Default|SetIndex _index)
    (Variables|Default|SetFinalTangentScale (select (== _index (.ReturnValue (Math|Float|Division(WholeandRemainder) (Spline|GetSplineLength (Variables|Default|GetMainSpline)) _spacing_2))) (* (/ (.Remainder (Math|Float|Division(WholeandRemainder) (Spline|GetSplineLength (Variables|Default|GetMainSpline)) _spacing_2)) _spacing_2) (Variables|Default|GetTangentScale)) (Variables|Default|GetTangentScale)))
    (bind _output_get_2 (Variables|Default|SetstartDistance (* (Variables|Default|GetIndex) _spacing)))
    (Variables|Default|SetMiddleDistance (+ _output_get_2 (* _spacing 0.5)))
    (Variables|Default|SetEndDistance (+ (Variables|Default|GetstartDistance) (Variables|Default|GetSpacing)))
    (bind _returnvalue_4 (AddComponent|AddSplineMeshComponent false))
    (SplineMesh|SetStartScale _returnvalue_4 (Math|Vector2D|MakeVector2D (* (Variables|Default|GetNewBranchThickness) _branchthickness) (* (Variables|Default|GetNewBranchThickness) _branchthickness)) true :!class /Script/Engine.SplineMeshComponent)
    (bind _output_get_3 (Variables|Default|SetNewBranchThickness (/ (- (* (Variables|Default|GetNewBranchThickness) _branchthickness) (/ 1.0 (* (Variables|Default|GetIndex) (Variables|Default|GetstartDistance)))) (Variables|Default|GetBranchThicknessRatio))))
    (SplineMesh|SetEndScale _returnvalue_4 (* (Math|Vector2D|MakeVector2D _output_get_3 _output_get_3) _branchthickness) true :!class /Script/Engine.SplineMeshComponent)
    (SplineMesh|SetForwardAxis _returnvalue_4 "X" true)
    (SplineMesh|SetStartandEnd _returnvalue_4 (Spline|GetLocationatDistanceAlongSpline (Variables|Default|GetMainSpline) (Variables|Default|GetstartDistance) "Local") (* (Spline|GetDirectionatDistanceAlongSpline (Variables|Default|GetMainSpline) (Variables|Default|GetstartDistance) "Local") (Variables|Default|GetFinalTangentScale)) (Spline|GetLocationatDistanceAlongSpline (Variables|Default|GetMainSpline) (Variables|Default|GetEndDistance) "Local") (* (Spline|GetDirectionatDistanceAlongSpline (Variables|Default|GetMainSpline) (Variables|Default|GetEndDistance) "Local") (Variables|Default|GetFinalTangentScale)) true :!class /Script/Engine.SplineMeshComponent)
    (if (<= (Math|Random|RandomFloatinRange 0.0 1e+02) (Variables|Default|GetBranch%20Probability))
      (Components|InstancedStaticMesh|AddInstance (Variables|Default|GetLeaf) (Math|Transform|MakeTransform (Spline|GetLocationatDistanceAlongSpline (Variables|Default|GetMainSpline) (Variables|Default|GetstartDistance) "Local"))))))

(fn GetSplinePoints
  (bind _controlspline (Variables|Default|GetControlSpline))
  (Utilities|Array|Clear (Variables|Default|GetSplinePoints))
  (for _index (range 0 (- (Spline|GetNumberOfSplinePoints _controlspline) 1))
    (Utilities|Array|SetArrayElem (Variables|Default|GetSplinePoints) _index (Utilities|Struct|MakeSplinePoint (Math|Conversions|ToFloat(Integer) _index) (.location (Spline|GetTransformatSplinePoint _controlspline _index "Local" true)) (Spline|GetArriveTangentatSplinePoint _controlspline _index "Local") (Spline|GetLeaveTangentatSplinePoint _controlspline _index "Local") (.rotation (Spline|GetTransformatSplinePoint _controlspline _index "Local" true)) (.scale (Spline|GetTransformatSplinePoint _controlspline _index "Local" true)) (Class|SplineComponent|GetSplinePointType _controlspline _index)) true)))