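; Spline-based scattering tool that places instanced meshes, presumably rocks given the asset name, along an editable path.
; The construction script steps along the spline at the Spacing interval and adds a Hierarchical Instanced Static Mesh instance at each point.
; A random stream gives each instance repeatable yaw and uniform scale variation, with pitch set by VerticalRotation.
; The event graph holds no active logic.
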(event EventBeginPlay)

(event Collision|EventActorBeginOverlap
  (params (OtherActor :type Actor%20Object%20Reference)))

(event EventTick
  (params (DeltaSeconds :type Float%20%28single-precision%29)))

(fn ConstructionScript
  (bind _spline (Variables|Default|GetSpline))
  (bind _spacing (Variables|Mesh|Getspacing))
  (bind _randomstream (Variables|Default|GetRandomStream))
  (for _index (range 0 (.ReturnValue (Math|Float|Division(WholeandRemainder) (Spline|GetSplineLength _spline) _spacing)))
    (Class|InstancedStaticMeshComponent|AddInstanceWorldSpace (Variables|Default|GetHierarchicalInstancedStaticMesh) (Math|Transform|MakeTransform (Spline|GetLocationatDistanceAlongSpline _spline (* (Math|Conversions|ToFloat(Integer) _index) _spacing) "World") (Math|Rotator|MakeRotator 0.0 (Variables|Mesh|GetVertical%20Rotation) (Math|Random|RandomFloatinRangefromStream 0.0 3.6e+02 _randomstream)) (Math|Conversions|ToVector(Float) (Math|Random|RandomFloatinRangefromStream (Variables|MeshSize|GetMin) (Variables|MeshSize|GetMax) _randomstream))))))