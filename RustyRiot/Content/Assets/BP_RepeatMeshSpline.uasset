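; BP_RepeatMeshSpline is a construction-script actor that repeats a mesh along a spline using instanced mesh components.
; It adds instances at spacing intervals with random extra spacing, a rotation offset and random rotation.
; A start cap sits at the first point and can repeat with each mesh.
; With VisualEditing off, the spline is rebuilt from the SplinePoints array and an end cap is added.
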(event EventBeginPlay)

(event Collision|EventActorBeginOverlap
  (params (OtherActor :type Actor%20Object%20Reference)))

(event EventTick
  (params (DeltaSeconds :type Float%20%28single-precision%29)))

(fn ConstructionScript
  (bind _spline (Variables|Default|GetSpline))
  (bind _random_rotation (Variables|Default|GetRandom%20Rotation))
  (bind _mesh_rotation (Variables|Default|GetMesh%20Rotation))
  (Components|StaticMesh|SetStaticMesh (Variables|Default|GetMesh%20Instance) (Variables|Default|GetMesh))
  (Components|StaticMesh|SetStaticMesh (Variables|Default|GetStart%20Cap%20Instance) (Variables|Default|GetStart%20Cap%20Mesh))
  (Components|StaticMesh|SetStaticMesh (Variables|Default|GetEnd%20Cap%20Instance) (Variables|Default|GetEnd%20Cap%20Mesh))
  (bind _output_get (LocalVariables|SetReapeatTransform (Spline|GetTransformatSplinePoint (Variables|Default|GetSpline) 0 "Local" false)))
  (Components|InstancedStaticMesh|AddInstance (Variables|Default|GetStart%20Cap%20Instance) _output_get)
  (if (Variables|Default|GetVisual%20Editing)
    _
    (else
      (Spline|SetSplinePoints (Variables|Default|GetSpline) (Variables|Default|GetSpline%20Points) "Local" true)
      (Components|InstancedStaticMesh|AddInstance (Variables|Default|GetEnd%20Cap%20Instance) (Spline|GetTransformatSplinePoint _spline (Spline|GetNumberOfSplinePoints _spline) "Local" false))))
  (for _index (range 0 (Math|Float|Floor (/ (Spline|GetSplineLength (Variables|Default|GetSpline)) (Variables|Default|GetMesh%20Spacing))))
    (bind _output_get_2 (LocalVariables|SetLocationOnSpline (* _index (+ (Math|Random|RandomFloatinRange 0.0 (Variables|Default|GetMesh%20Random%20Extra%20Spacing)) (Variables|Default|GetMesh%20Spacing)))))
    (bind _output_get_3 (LocalVariables|SetReapeatTransform (Math|Transform|MakeTransform (.location (Spline|GetTransformatDistanceAlongSpline (Variables|Default|GetSpline) _output_get_2 "Local" false)) (Math|Rotator|CombineRotators (Math|Rotator|MakeRotator (.x _mesh_rotation) (.y _mesh_rotation) (.z _mesh_rotation)) (Math|Rotator|CombineRotators (.rotation (Spline|GetTransformatDistanceAlongSpline (Variables|Default|GetSpline) _output_get_2 "Local" false)) (Math|Rotator|MakeRotator (Math|Random|RandomFloatinRange (* (.x _random_rotation) -1.0) (.x _random_rotation)) (Math|Random|RandomFloatinRange (* (.y _random_rotation) -1.0) (.y _random_rotation)) (Math|Random|RandomFloatinRange (* (.z _random_rotation) -1.0) (.z _random_rotation))))) (.scale (Spline|GetTransformatDistanceAlongSpline (Variables|Default|GetSpline) _output_get_2 "Local" false)))))
    (Components|InstancedStaticMesh|AddInstance (Variables|Default|GetMesh%20Instance) _output_get_3)
    (if (Variables|Default|GetRepeat%20Start%20Cap)
      (Components|InstancedStaticMesh|AddInstance (Variables|Default|GetStart%20Cap%20Instance) (LocalVariables|GetReapeatTransform)))))